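; GA_RockLeap is a charged gameplay ability that launches the avatar character in a leap toward the mouse position.
; On full charge, it takes the 2D direction to the cursor and uses the distance, clamped between MinJump and MaxRange, directly as horizontal launch speed.
; The launch overrides XY velocity and adds a fixed upward impulse, then OnFullChargeComplete is called.
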(event `self.OnFullCharge`
  (bind _returnvalue (`self.GetAvatarActorFromActorInfo`))
  (bind _minjump (`self.MinJump`))
  (bind _maxrange (`self.MaxRange`))
  (bind _aspawn (cast `Pawn` _returnvalue))
  (bind _newparam (`self.GetMousePosition`))
  (bind _ascharacter (cast `Character` _returnvalue))
  (bind _location (.location (`Actor.GetTransform` _aspawn)))
  (bind _returnvalue_2 (`KismetMathLibrary.Vector_Distance2D` _newparam _location))
  (if (< _returnvalue_2 _minjump)
    (bind _returnvalue_3 (`KismetMathLibrary.Normal2D` (`KismetMathLibrary.MakeVector2D` (.x (- _newparam _location)) (.y (- _newparam _location)))))
    (bind (_x _y) (`KismetMathLibrary.BreakVector2D` (* _returnvalue_3 _minjump)))
    (`Character.LaunchCharacter` _ascharacter (`KismetMathLibrary.MakeVector` _x _y 500.0) true false)
    (elif (> _returnvalue_2 _maxrange)
      (bind (_x_2 _y_2) (`KismetMathLibrary.BreakVector2D` (* _returnvalue_3 _maxrange)))
      (`Character.LaunchCharacter` _ascharacter (`KismetMathLibrary.MakeVector` _x_2 _y_2 500.0) true false)
      (else
        (bind (_x_3 _y_3) (`KismetMathLibrary.BreakVector2D` (* _returnvalue_3 _returnvalue_2)))
        (`Character.LaunchCharacter` _ascharacter (`KismetMathLibrary.MakeVector` _x_3 _y_3 500.0) true false))))
  (`self.OnFullCharge Complete`))