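; Actor component for a multi-kill ability that destroys several targeted actors at once.
; While charging, Tick calls the player character's multi-object targeting within a fixed range, passing the MultiTarget array, and draws a circular target zone at the result.
; Execution destroys every valid actor in MultiTarget and returns true, or false if the array is empty.
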(event `self.ReceiveTick`
  (params (DeltaSeconds :type "Float (single-precision)"))
  (if (`self.Charging`)
    (bind _location (`/Game/Blueprints/SimplePlayerCharacter.TargetMultipleObject` (`self.PlayerCharacter`) 2000.0 0.0 0.0 (`|MakeArray` "ObjectTypeQuery7" :!type "EObjectTypeQuery Enum") (`self.multiTarget`) false))
    (`/Game/Blueprints/SimplePlayerCharacter.DrawTargetedZone` (`self.PlayerCharacter`) "ArrowMaterial" (`|MakeMap` "radius" 300) "sphere" _location)))

(fn `Execution`
  (returns (executed :type Boolean))
  (if (!= (`KismetArrayLibrary.Array_Length` (`self.multiTarget`)) 0)
    ;[1 1 1] kill every actor in the array
    (for _array_element (`self.multiTarget`)
      (`/Engine/EditorBlueprintResources/StandardMacros.IsValid` _array_element
        (:`Is Valid`
          (`Actor.K2_DestroyActor` _array_element))))
    (return true)
    (else
      (return false))))