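; Multi-kill skill component that destroys several targeted actors at once.
; While charging, Tick calls the player character's multi-object targeting with a range limit and object type filter, passing MultiTarget as the previous targets.
; Execution destroys every valid actor in MultiTarget and returns true, or returns false when the array is empty.
; A disconnected branch for destroying a MultipleTargetZone component never runs.
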(event `self.ReceiveTick`
  (params (DeltaSeconds :type "Float (single-precision)"))
  (if (`self.Charging`)
    (`/Game/Blueprints/mergeAsset.TargetMultipleObject` (`self.PlayerCharacter`) 2000.0 0.0 0.0 (`|MakeArray` "ObjectTypeQuery7" :!type "EObjectTypeQuery Enum") (`self.multiTarget`) false)))

(fn `Execution`
  (returns (executed :type Boolean))
  (`KismetSystemLibrary.PrintString` "Execution for multiple target")
  (if (!= (`KismetArrayLibrary.Array_Length` (`self.multiTarget`)) 0)
    ;[1 1 1] kill every actor in the array
    (for _array_element (`self.multiTarget`)
      (`/Engine/EditorBlueprintResources/StandardMacros.IsValid` _array_element
        (:`Is Valid`
          (`Actor.K2_DestroyActor` _array_element))))
    (return true)
    (else
      (`KismetSystemLibrary.PrintString` "no target for multikill")
      (return false))))