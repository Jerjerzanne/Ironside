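; BaseSkill is an actor component for a charge-and-release player skill that destroys a single targeted actor.
; While charging, Tick runs the player character's individual-object targeting, and a timer forces release at the maximum cast time.
; Release with a valid target destroys it, starts a timed cooldown on CanCastSkill and schedules the character's return to idle.
; Release without a target returns the character to idle immediately.
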(event `self.ReceiveTick`
  (params (DeltaSeconds :type "Float (single-precision)"))
  (if (`self.Charging`)
    (`/Game/Blueprints/SimplePlayerCharacter.TargetIndividualObject` (`self.PlayerCharacter`) (`|MakeArray` "ObjectTypeQuery7" :!type "EObjectTypeQuery Enum") (`self.SingleTarget`) 2000.0 25.0)))

(event `self.ReceiveBeginPlay`
  (bind _assimple_player_character (cast `/Game/Blueprints/SimplePlayerCharacter` (`GameplayStatics.GetPlayerCharacter` 0))
    (:`then`
      (set `self.PlayerCharacter` _assimple_player_character))
    (:`CastFailed`
      (`KismetSystemLibrary.PrintString` "Skill has failed to attach player"))))

(fn `RefreshCooldown`
  (bind _cooldowntimer (`self.CooldownTimer`))
  (set `self.CanCastSkill` true)
  (`KismetSystemLibrary.PrintString` "refreshed cooldown")
  (if (`KismetSystemLibrary.K2_IsTimerActiveHandle` _cooldowntimer)
    (`KismetSystemLibrary.K2_ClearAndInvalidateTimerHandle` _cooldowntimer)))

(fn `SetCooldown`
  (bind _maxcooldown (`self.MaxCooldown`))
  (set `self.CooldownDuration` _maxcooldown)
  (bind _returnvalue (`KismetSystemLibrary.K2_SetTimer` null "RefreshCooldown" _maxcooldown))
  (set `self.CooldownTimer` _returnvalue))

(fn `StartCharge`
  (set `self.Charging` true)
  (bind _returnvalue (`KismetSystemLibrary.K2_SetTimer` null "StartRelease" (`self.MaxCastTime`)))
  (set `self.ChargeTimer` _returnvalue))

(fn `StartRelease`
  (bind _playercharacter (`self.PlayerCharacter`))
  (bind _chargetimer (`self.ChargeTimer`))
  (bind _singletarget (`self.SingleTarget`))
  (set `self.Charging` false)
  (if (`KismetSystemLibrary.K2_IsTimerActiveHandle` _chargetimer)
    (`KismetSystemLibrary.K2_ClearAndInvalidateTimerHandle` _chargetimer))
  (`/Engine/EditorBlueprintResources/StandardMacros.IsValid` _singletarget
    (:`Is Valid`
      (`KismetSystemLibrary.PrintString` "kill")
      (`Actor.K2_DestroyActor` _singletarget)
      (set `self.CanCastSkill` false)
      (`self.SetCooldown`)
      (bind _returnvalue (`KismetSystemLibrary.K2_SetTimer` _playercharacter "ReturnToIdle" (`self.ReleaseToIdleTime`)))
      (set `self.ReleaseTimer` _returnvalue))
    (:`Is Not Valid`
      (`/Game/Blueprints/SimplePlayerCharacter.ReturnToIdle` _playercharacter))))