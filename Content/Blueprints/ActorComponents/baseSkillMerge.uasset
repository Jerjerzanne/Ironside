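; Base actor component for a player skill, handling charge, release and cooldown on the SimplePlayerCharacter cached at BeginPlay.
; StartCharge runs a cast timer leading to StartRelease, which calls Execution if that timer is still active and removes the player's target zone.
; A successful Execution starts the cooldown and an optional delay before idle, while failure returns to idle immediately.
; Execution returns false here, serving as the hook for child skills.
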(event `self.ReceiveBeginPlay`
  (bind _assimple_player_character (cast `/Game/Blueprints/SimplePlayerCharacter` (`GameplayStatics.GetPlayerCharacter` 0))
    (:`then`
      (set `self.PlayerCharacter` _assimple_player_character))
    (:`CastFailed`
      (`KismetSystemLibrary.PrintString` "Skill has failed to attach player"))))

(fn `Execution`
  (returns (executed :type Boolean))
  (return false))

(fn `RefreshCooldown`
  (bind _cooldowntimer (`self.CooldownTimer`))
  (set `self.CanCastSkill` true)
  (`KismetSystemLibrary.PrintString` "refreshed cooldown")
  (if (`KismetSystemLibrary.K2_IsTimerActiveHandle` _cooldowntimer)
    (`KismetSystemLibrary.K2_ClearAndInvalidateTimerHandle` _cooldowntimer)))

(fn `SetCooldown`
  (bind _maxcooldown (`self.MaxCooldown`))
  (set `self.CooldownDuration` _maxcooldown)
  (if (< 0.0 _maxcooldown)
    (bind _returnvalue (`KismetSystemLibrary.K2_SetTimer` null "RefreshCooldown" _maxcooldown))
    (set `self.CooldownTimer` _returnvalue)
    (else
      (`self.RefreshCooldown`))))

(fn `StartCharge`
  (bind _maxcasttime (`self.MaxCastTime`))
  (set `self.Charging` true)
  (if (< 0.0 _maxcasttime)
    (bind _returnvalue (`KismetSystemLibrary.K2_SetTimer` null "StartRelease" _maxcasttime))
    (set `self.ChargeTimer` _returnvalue)
    (else
      (`self.StartRelease`))))

(fn `StartRelease`
  (bind _playercharacter (`self.PlayerCharacter`))
  (bind _releasetoidletime (`self.ReleaseToIdleTime`))
  (bind _playercharacter_2 (`self.PlayerCharacter`))
  (bind _chargetimer (`self.ChargeTimer`))
  (set `/Game/Blueprints/SimplePlayerCharacter.CurrentState` "NewEnumerator2" (`self.PlayerCharacter`))
  (set `self.Charging` false)
  (if (`KismetSystemLibrary.K2_IsTimerActiveHandle` _chargetimer)
    (`KismetSystemLibrary.K2_ClearAndInvalidateTimerHandle` _chargetimer)
    (bind _executed (`self.Execution`))
    (`/Game/Blueprints/SimplePlayerCharacter.DestroyTargetZone` _playercharacter (`/Game/Blueprints/SimplePlayerCharacter.multipleTargetZone` _playercharacter))
    (if _executed
      ;[1 1 1] Set cooldown of the skill
      (set `self.CanCastSkill` false)
      (`self.SetCooldown`)
      (if (< 0.0 _releasetoidletime)
        (bind _returnvalue (`KismetSystemLibrary.K2_SetTimer` _playercharacter_2 "ReturnToIdle" _releasetoidletime))
        (set `self.ReleaseTimer` _returnvalue)
        (else
          (`/Game/Blueprints/SimplePlayerCharacter.ReturnToIdle` _playercharacter_2)))
      (else
        ;[1 1 1] dont set off cooldown
        (`/Game/Blueprints/SimplePlayerCharacter.ReturnToIdle` (`self.PlayerCharacter`))))))