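; Skill actor component that kills a single targeted object by destroying its actor.
; While charging, Tick asks the player character to retarget among one object type, passing the current single target as the previous one.
; Execution destroys that target if it is valid and returns whether it succeeded.
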(event `self.ReceiveTick`
  (params (DeltaSeconds :type "Float (single-precision)"))
  (if (`self.Charging`)
    (`/Game/Blueprints/mergeAsset.TargetIndividualObject` (`self.PlayerCharacter`) (`|MakeArray` "ObjectTypeQuery7" :!type "EObjectTypeQuery Enum") (`self.SingleTarget`) 2000.0 25.0)))

(fn `Execution`
  (returns (executed :type Boolean))
  (bind _singletarget (`self.SingleTarget`))
  (`/Engine/EditorBlueprintResources/StandardMacros.IsValid` _singletarget
    (:`Is Valid`
      (`Actor.K2_DestroyActor` _singletarget)
      (return true))
    (:`Is Not Valid`
      (return false))))