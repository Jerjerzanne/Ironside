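; Game mode that gates match start until the player count equals the maximum and an all-players-ready flag is set.
; PostLogin records each controller and switches its view to a shared camera when that reference is valid.
; Player starts are drawn randomly without repeats from a cached list, refilled from the level when empty.
; Tick prints player-count and match-state debug text on screen.
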(event `self.ReceiveTick`
  (params (DeltaSeconds :type "Float (single-precision)"))
  (`KismetSystemLibrary.PrintString` (`KismetStringLibrary.JoinStringArray` (`|MakeArray` "NumPlayers:" (`KismetStringLibrary.Conv_IntToString` (`self.NumPlayers`)))) true true (struct :`G` 0.66 :`B` 1.0 :`A` 1.0) 0.0)
  (`KismetSystemLibrary.PrintString` (`KismetStringLibrary.Conv_NameToString` (`self.GetMatchState`)) true true (struct :`G` 0.66 :`B` 1.0 :`A` 1.0) 0.0))

(event `self.K2_PostLogin`
  (params (NewPlayer :type "PlayerController Object Reference"))
  (bind _camera (`self.Camera`))
  (`KismetArrayLibrary.Array_Add` (`self.PlayerControllerList`) NewPlayer)
  (`/Engine/EditorBlueprintResources/StandardMacros.IsValid` _camera
    (:`Is Valid`
      (`PlayerController.SetViewTargetWithBlend` NewPlayer _camera 0.0 "VTBlend_Linear" 0.0 false))))

(fn `ChoosePlayerStart`
  (params (Player :type "Controller Object Reference"))
  (returns (ReturnValue :type "Actor Object Reference"))
  (bind _playerstarts (`self.PlayerStarts`))
  (bind _returnvalue (`KismetArrayLibrary.Array_Length` _playerstarts))
  (if (== _returnvalue 0)
    (bind _outactors (`GameplayStatics.GetAllActorsOfClass` "/Script/Engine.PlayerStart"))
    (set `self.PlayerStarts` _outactors))
  (bind _output_get (set `self.SelectedPlayerStart` (`|GetArrayItem` _playerstarts (`KismetMathLibrary.RandomInteger` _returnvalue))))
  (`KismetArrayLibrary.Array_RemoveItem` _playerstarts _output_get)
  (return (`self.SelectedPlayerStart`)))

(fn `ReadyToStartMatch`
  (returns (ReturnValue :type Boolean))
  (return (and (== (`self.MaxNumPlayers`) (`self.NumPlayers`)) (`self.AllPlayersReady`))))

(fn `UserConstructionScript`)