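; Game state that tracks player readiness and reports it to OldGameMode.
; Every tick it loops PlayerArray, prints each TopDownPlayerState's ID and ready flag, and sets the game mode's AllPlayersReady when none are unready.
; The flag is only ever set to true on the game mode, never cleared.
; A separate PlayerAcknowledge event prints and stores controller IDs in PlayersReadyList, which the tick check ignores.
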(event `self.ReceiveTick`
  (params (DeltaSeconds :type "Float (single-precision)"))
  (set `self.AllPlayersReady` true)
  (for _array_element (`self.PlayerArray`)
    (bind _astop_down_player_state (cast `/Game/Blueprints/Characters/TopDownPlayerState` _array_element))
    (bind _playerready (`/Game/Blueprints/Characters/TopDownPlayerState.PlayerReady` _astop_down_player_state))
    (`KismetSystemLibrary.PrintString` (`KismetStringLibrary.Concat_StrStr` (`KismetStringLibrary.Conv_IntToString` (`PlayerState.PlayerId` _astop_down_player_state)) ": " (`KismetStringLibrary.Conv_BoolToString` _playerready)) true true (struct :`R` 1.0 :`B` 0.068094 :`A` 1.0) 0.0)
    (if (not _playerready)
      (set `self.AllPlayersReady` false)))
  (if (`self.AllPlayersReady`)
    (bind _asold_game_mode (cast `/Game/Blueprints/GameModes/OldGameMode` (`self.AuthorityGameMode`)))
    (set `/Game/Blueprints/GameModes/OldGameMode.AllPlayersReady` true _asold_game_mode)))

(event `PlayerAcknowledge`
  (params (PlayerControllerID :type Integer))
  (`KismetSystemLibrary.PrintString` (`KismetStringLibrary.Conv_IntToString` PlayerControllerID) true true (struct :`R` 1.0 :`G` 0.03269 :`A` 1.0))
  (`KismetArrayLibrary.Array_Add` (`self.PlayersReadyList`) PlayerControllerID))

(fn `UserConstructionScript`)