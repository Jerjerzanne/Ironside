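; BaseMeleeAttack is a short-lived moving hit actor that deals melee damage to what it overlaps.
; Each tick it sweeps along world negative Y at AttackSpeed and accumulates TimeActive, destroying itself once that exceeds AttackLifespan.
; On overlap it passes MeleeDamage through TakeDamage to actors implementing DamageInterface, and stays alive after a hit.
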(event `self.ReceiveTick`
  (params (DeltaSeconds :type "Float (single-precision)"))
  (bind _timeactive (`self.TimeActive`))
  ;[1 1 1] Check lifespan
  (if (> _timeactive (`self.AttackLifespan`))
    (`self.K2_DestroyActor`)
    (else
      (set `self.TimeActive` (+ DeltaSeconds _timeactive))
      ;[1 1 1] Move attack collider
      (`self.K2_SetActorLocation` (+ (* (0.0 -1.0 0.0) (* DeltaSeconds (`self.AttackSpeed`))) (`self.K2_GetActorLocation`)) true))))

(event `self.ReceiveActorBeginOverlap`
  (params (OtherActor :type "Actor Object Reference"))
  (bind _asdamage_interface (cast `/Game/Interfaces/DamageInterface` OtherActor))
  (`/Game/Blueprints/EnemyCharacters/BaseEnemyCharacter.TakeDamage` _asdamage_interface (`self.MeleeDamage`)))

(fn `UserConstructionScript`)