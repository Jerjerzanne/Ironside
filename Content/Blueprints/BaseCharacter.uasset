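; Base character Blueprint with health, skill charging and mouse-aimed rotation.
; BeginPlay fills health and applies a base-stats Gameplay Effect; damage reduces health and destroys the actor at zero.
; An enum state and current skill gate charge and release calls on skill objects.
; Tick projects player 0's cursor onto a horizontal plane; RotatePlayer faces that point locally, then passes the rotation to SetRotationServer.
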(event `SetRotationServer`
  (params (Target :type "Actor Object Reference") (NewRotation :type "Rotator Structure"))
  ;[1 1 1] Managing Server/Client communication
  (`self.K2_SetActorRotation` Target NewRotation false))

(event `self.ReceiveBeginPlay`
  ;[1 1 1] BeginPlay
  (`self.SetHealthToMax`)
  (`AbilitySystemComponent.BP_ApplyGameplayEffectToSelf` :`self` (`self.AbilitySystem`) :`GameplayEffectClass` "/Game/Blueprints/GameplayAbilities/GE_StatsBase.GE_StatsBase_C" :`Level` 1.0))

(event `self.ReceiveTick`
  (params (DeltaSeconds :type "Float (single-precision)"))
  ;[1 1 1] Tick
  (`self.GetMousePosition`))

(event `/Game/Interfaces/DamageInterface.TakeDamage`
  (params (Damage :type Integer))
  ;[1 1 1] Override the damage interface
  (bind _output_get (set `self.CurrentHealth` (- (`self.CurrentHealth`) Damage)))
  (if (<= _output_get 0)
    (`/Game/Interfaces/DamageInterface.Die`)))

(event `/Game/Interfaces/DamageInterface.Die`
  ;[1 1 1] Override the damage interface
  (`self.K2_DestroyActor`))

(fn `DrawCircleAreaEffect`)

(fn `DrawMouseLocation`
  (params (HasBeenDrawn :type "Boolean (by ref)"))
  (if HasBeenDrawn
    (bind _returnvalue (`WidgetLayoutLibrary.GetMousePositionOnViewport`))
    (`SceneComponent.K2_SetWorldLocation` (`self.mouseComponent`) (`KismetMathLibrary.Conv_Vector2DToVector` _returnvalue) false false)
    (else
      (bind _returnvalue_2 (`AddComponent|NODE_AddStaticMeshComponent-3`))
      (set `self.mouseComponent` _returnvalue_2))))

(fn `FindMouseLocation`)

(fn `GetMousePosition`
  (bind _returnvalue (`GameplayStatics.GetPlayerController` 0))
  (bind (_worldlocation _worlddirection _returnvalue_2) (`PlayerController.DeprojectMousePositionToWorld` _returnvalue))
  (bind _returnvalue_3 (`PlayerCameraManager.GetCameraLocation` (`PlayerController.PlayerCameraManager` _returnvalue)))
  (if _returnvalue_2
    (set `self.MousePosition` (`.Intersection` (`KismetMathLibrary.LinePlaneIntersection_OriginNormal` _returnvalue_3 (+ (* (- _worldlocation _returnvalue_3) 251.0) _worldlocation) (0.0 0.0 0.0) (0.0 0.0 1.0))))))

(fn `ReturnToIdle`
  (set `self.CurrentState` "NewEnumerator0")
  (set `self.CurrentSkill` null)
  (set `self.ChargePercentage` 0.0))

(fn `RotatePlayer`
  (bind _returnvalue (`Controller.K2_GetPawn` (`GameplayStatics.GetPlayerController` 0)))
  (bind _returnvalue_2 (`KismetMathLibrary.FindLookAtRotation` (`KismetMathLibrary.MakeVector` (.x (`self.K2_GetActorLocation` _returnvalue)) (.y (`self.K2_GetActorLocation` _returnvalue))) (`self.MousePosition`)))
  (`self.K2_SetActorRotation` _returnvalue _returnvalue_2 false)
  (`self.SetRotationServer` _returnvalue _returnvalue_2))

(fn `SetHealthToMax`
  (set `self.CurrentHealth` (`self.MaxHealth`)))

(fn `TryCharging`
  (params (skill :type "/Game/Blueprints/Skills/BaseSkill Object Reference (by ref)"))
  (if (`|EnumEquality` (`self.CurrentState`) "NewEnumerator0")
    (if (`/Game/Blueprints/Skills/BaseSkill.CanCastSkill` skill)
      (set `self.CurrentState` "NewEnumerator1")
      (set `self.CurrentSkill` skill)
      (`/Game/Blueprints/Skills/BaseSkill.StartCharge` skill))))

(fn `TryRelease`
  (params (Skill :type "/Game/Blueprints/Skills/BaseSkill Object Reference (by ref)"))
  (if (`|EnumEquality` (`self.CurrentState`) "NewEnumerator1")
    (`/Game/Blueprints/Skills/BaseSkill.StartRelease` Skill false)))

(fn `UserConstructionScript`)