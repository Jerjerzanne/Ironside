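; Player character Blueprint with sprint, crouch, first/third-person camera toggle and interaction through BaseInteractable.
; Camera toggle moves the camera between placement components and swaps overlap collision between Capsule and InteractTriggerZone.
; Overlaps toggle custom-depth highlighting on the other actor's static mesh.
; Sphere-trace functions pick the closest interactable or individual, but their calls are unwired, so nothing running sets the target Interact uses.
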(event `InputAction|Interact`
  (params (Key :type "Key Structure"))
  (bind _interactabletarget (`self.InteractableTarget`))
  ;[1 1 1] Interact
  (:`Pressed`
    (`/Engine/EditorBlueprintResources/StandardMacros.IsValid` _interactabletarget
      (:`Is Valid`
        (`self.Interact` _interactabletarget)))))

(event `self.ReceiveTick`
  (params (DeltaSeconds :type "Float (single-precision)")))

(event `OnFirstPerson`
  ;[1 1 1] Events for first and third camera
  (`SceneComponent.K2_SetRelativeLocation` (`self.Camera`) (.location (`SceneComponent.GetRelativeTransform` (`self.FirstCameraPlacement`))) false false)
  (`SceneComponent.K2_SetRelativeRotation` :`self` (`self.Camera`))
  (`PrimitiveComponent.SetCollisionEnabled` (`self.Capsule`) "QueryAndPhysics")
  (`PrimitiveComponent.SetCollisionEnabled` (`self.InteractTriggerZone`) "NoCollision"))

(event `InputAction|Sprint`
  (params (Key :type "Key Structure"))
  ;[1 1 1] Sprint System
  (:`Pressed`
    (if (`self.CanSprint`)
      (`self.OnStartSprinting` (`self.SprintMovementSpeed`))
      (set `self.IsSprinting` true)))
  (:`Released`
    (if (`self.IsSprinting`)
      (`self.OnStopSprinting` (`self.BaseMovementSpeed`))
      (set `self.IsSprinting` false))))

(event `OnThirdPerson`
  ;[1 1 1] Events for first and third camera
  (`SceneComponent.K2_SetRelativeLocation` (`self.Camera`) (.location (`SceneComponent.GetRelativeTransform` (`self.ThirdCameraPlacement`))) false false)
  (`SceneComponent.K2_SetRelativeRotation` (`self.Camera`) (struct :`Pitch` -20.0) false false)
  (`PrimitiveComponent.SetCollisionEnabled` (`self.InteractTriggerZone`) "QueryAndPhysics")
  (`PrimitiveComponent.SetCollisionEnabled` (`self.Capsule`) "NoCollision"))

(event `OnStartSprinting`
  (params (SprintVelocity :type "Float (double-precision)"))
  ;[1 1 1] Sprint System
  (set `CharacterMovementComponent.MaxWalkSpeed` SprintVelocity (`self.CharacterMovement`)))

(event `OnStopSprinting`
  (params (BaseVelocity :type "Float (double-precision)"))
  ;[1 1 1] Sprint System
  (set `CharacterMovementComponent.MaxWalkSpeed` BaseVelocity (`self.CharacterMovement`)))

(event `InputAction|Crouch`
  (params (Key :type "Key Structure"))
  ;[1 1 1] Crouching System
  (:`Pressed`
    (`self.Crouch`))
  (:`Released`
    (`self.UnCrouch`)))

(event `InputAction|ToggleCamera`
  (params (Key :type "Key Structure"))
  ;[1 1 1] Trigger for first or third camera
  (:`Pressed`
    (if (`self.isFirstPerson`)
      (set `self.isFirstPerson` false)
      (`self.OnThirdPerson`)
      (else
        (set `self.isFirstPerson` true)
        (`self.OnFirstPerson`)))))

(event `self.Capsule.OnComponentBeginOverlap`
  (params (OverlappedComponent :type "PrimitiveComponent Object Reference") (OtherActor :type "Actor Object Reference") (OtherComp :type "PrimitiveComponent Object Reference") (OtherBodyIndex :type Integer) (bFromSweep :type Boolean) (SweepResult :type "HitResult Structure (by ref)"))
  ;[1 1 1] Interactable Trigger Zone
  (`self.ToggleHighlight` OtherActor))

(event `self.Capsule.OnComponentEndOverlap`
  (params (OverlappedComponent :type "PrimitiveComponent Object Reference") (OtherActor :type "Actor Object Reference") (OtherComp :type "PrimitiveComponent Object Reference") (OtherBodyIndex :type Integer))
  ;[1 1 1] Interactable Trigger Zone
  (`self.ToggleHighlight` OtherActor))

(event `self.InteractTriggerZone.OnComponentBeginOverlap`
  (params (OverlappedComponent :type "PrimitiveComponent Object Reference") (OtherActor :type "Actor Object Reference") (OtherComp :type "PrimitiveComponent Object Reference") (OtherBodyIndex :type Integer) (bFromSweep :type Boolean) (SweepResult :type "HitResult Structure (by ref)"))
  ;[1 1 1] Interactable Trigger Zone
  (`self.ToggleHighlight` OtherActor))

(event `self.InteractTriggerZone.OnComponentEndOverlap`
  (params (OverlappedComponent :type "PrimitiveComponent Object Reference") (OtherActor :type "Actor Object Reference") (OtherComp :type "PrimitiveComponent Object Reference") (OtherBodyIndex :type Integer))
  ;[1 1 1] Interactable Trigger Zone
  (`self.ToggleHighlight` OtherActor))

(fn `FindClosestTarget`
  (params (HitsArray :type "Array of HitResult Structure"))
  (returns (HitActor :type "Actor Object Reference"))
  (locals (DistanceArray :type "Array of Float (double-precision)"))
  (for _array_element HitsArray
    ;[1 1 1] Add all distances to DistanceArray
    (`KismetArrayLibrary.Array_Add` (`local.DistanceArray`) (`.Distance` (`GameplayStatics.BreakHitResult` _array_element))))
  (return (`.HitActor` (`GameplayStatics.BreakHitResult` (`|GetArrayItem` (`local.HitsArray`) (`KismetMathLibrary.MinOfFloatArray` (`local.DistanceArray`)))))))

(fn `Interact`
  (params (InteractableTarget :type "Actor Object Reference"))
  (bind _asbase_interactable (cast `BaseInteractable` InteractableTarget)
    (:`then`
      (`BaseInteractable.RespondInteract` _asbase_interactable self))
    (:`CastFailed`
      (`KismetSystemLibrary.PrintString` "Error in Interact "))))

(fn `ShperecastByObject`
  (params (ObjectType :type "Array of EObjectTypeQuery Enum (by ref)" :default _))
  (returns (OutHits :type "Array of HitResult Structure") (ReturnValue :type Boolean))
  (bind _camera (`self.Camera`))
  (bind _returnvalue (`SceneComponent.K2_GetComponentLocation` _camera))
  ;[1 1 1] Cast a sphere in front of the camera
  (bind (_outhits _returnvalue_2) (`KismetSystemLibrary.SphereTraceMultiForObjects` _returnvalue (+ _returnvalue (* (`SceneComponent.GetForwardVector` _camera) (`self.DetectionRange`))) (`self.SpherecastRadius`) ObjectType))
  (return _outhits _returnvalue_2))

(fn `TargetIndividual`
  (returns (Target :type "Actor Object Reference"))
  (locals (NewTarget :type "Actor Object Reference"))
  (bind _newtarget (`local.NewTarget`))
  (bind _enemytarget (`self.EnemyTarget`))
  (bind _enemytarget_2 (`self.EnemyTarget`))
  (bind (_outhits _returnvalue) (`self.ShperecastByObject` (`|MakeArray` "ObjectTypeQuery7" :!type "EObjectTypeQuery Enum")))
  (if _returnvalue
    (bind _hitactor (`self.FindClosestTarget` _outhits))
    (set `local.NewTarget` _hitactor)
    ;[1 1 1] sets current target to new target, highlights it and removes highlight of the old target
    (`/Engine/EditorBlueprintResources/StandardMacros.IsValid` _enemytarget
      (:`Is Valid`
        (if (not (== _newtarget _enemytarget))
          (`self.ToggleHighlight` _enemytarget)
          (bind _output_get (set `self.EnemyTarget` _newtarget :!label _label))
          (`self.ToggleHighlight` _output_get)))
      (:`Is Not Valid`
        (goto _label)))
    (return _output_get)
    (else
      ;[1 1 1] No valid hit target - remove highlight from current target
      (`/Engine/EditorBlueprintResources/StandardMacros.IsValid` _enemytarget_2
        (:`Is Valid`
          (`self.ToggleHighlight` _enemytarget_2)
          (set `self.EnemyTarget` null)
          (return null))))))

(fn `TargetInteractable`
  (returns (Target :type "Actor Object Reference"))
  (locals (NewInteractable :type "Actor Object Reference"))
  (bind _interactabletarget (`self.InteractableTarget`))
  (bind _interactabletarget_2 (`self.InteractableTarget`))
  (bind _newinteractable (`local.NewInteractable`))
  (bind (_outhits _returnvalue) (`self.ShperecastByObject` (`|MakeArray` "ObjectTypeQuery8" :!type "EObjectTypeQuery Enum")))
  (if _returnvalue
    (bind _hitactor (`self.FindClosestTarget` _outhits))
    (set `local.NewInteractable` _hitactor)
    ;[1 1 1] sets current target to new target, highlights it and removes highlight of the old target
    (`/Engine/EditorBlueprintResources/StandardMacros.IsValid` _interactabletarget_2
      (:`Is Valid`
        (if (not (== _newinteractable _interactabletarget_2))
          (`self.ToggleHighlight` _interactabletarget_2)
          (bind _output_get (set `self.InteractableTarget` _newinteractable :!label _label))
          (`self.ToggleHighlight` _output_get)))
      (:`Is Not Valid`
        (goto _label)))
    (return _output_get)
    (else
      ;[1 1 1] No valid hit target - remove highlight from current target
      (`/Engine/EditorBlueprintResources/StandardMacros.IsValid` _interactabletarget
        (:`Is Valid`
          (`self.ToggleHighlight` _interactabletarget)
          (set `self.InteractableTarget` null)
          (return null))))))

(fn `ToggleHighlight`
  (params (Actor :type "Actor Object Reference"))
  (bind _returnvalue (`self.GetComponentByClass` Actor "/Script/Engine.StaticMeshComponent"))
  (`/Engine/EditorBlueprintResources/StandardMacros.IsValid` _returnvalue
    (:`Is Valid`
      (if (`PrimitiveComponent.bRenderCustomDepth` _returnvalue)
        (`PrimitiveComponent.SetRenderCustomDepth` _returnvalue false)
        (else
          (`PrimitiveComponent.SetRenderCustomDepth` _returnvalue true))))))

(fn `UserConstructionScript`)