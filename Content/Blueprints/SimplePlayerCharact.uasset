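; Player character with sprint, crouch, a first/third-person camera toggle, interaction and two charge-and-release skills.
; Skill input drives a state enum and the KillSk and MultiKillSk components; interaction calls RespondInteract on the current BaseInteractable target.
; Camera-based traces pick single targets or an area marked by a runtime mesh, with custom-depth highlighting.
; Tick is empty and this graph never runs the targeting functions; only the first-person interact zone tracks overlaps.
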(event `InputAction|Skill2`
  (params (Key :type "Key Structure"))
  (bind _multipletargetzone (`self.multipleTargetZone`))
  ;[1 1 1] Managing skill 2 input
  (:`Pressed`
    (if (`|EnumEquality` (`self.CurrentState`) "NewEnumerator0")
      (if (`/Game/Blueprints/ActorComponents/BaseSkill.CanCastSkill` (`self.multiKill_sk`))
        (set `self.CurrentState` "NewEnumerator1")
        (`/Game/Blueprints/ActorComponents/BaseSkill.StartCharge` (`self.multiKill_sk`)))))
  (:`Released`
    (set `self.hasBeenDrawn` false)
    (`/Engine/EditorBlueprintResources/StandardMacros.IsValid` _multipletargetzone
      (:`Is Valid`
        (`ActorComponent.K2_DestroyComponent` _multipletargetzone))
      (:`Is Not Valid`
        _))
    (if (`|EnumEquality` (`self.CurrentState`) "NewEnumerator1")
      (set `self.CurrentState` "NewEnumerator2")
      (`/Game/Blueprints/ActorComponents/BaseSkill.StartRelease` (`self.multiKill_sk`)))))

(event `InputAction|Skill1`
  (params (Key :type "Key Structure"))
  ;[1 1 1] Managing skill 1 input
  (:`Pressed`
    (if (`|EnumEquality` (`self.CurrentState`) "NewEnumerator0")
      (if (`/Game/Blueprints/ActorComponents/BaseSkill.CanCastSkill` (`self.kill_sk`))
        (set `self.CurrentState` "NewEnumerator1")
        (`/Game/Blueprints/ActorComponents/BaseSkill.StartCharge` (`self.kill_sk`)))))
  (:`Released`
    (if (`|EnumEquality` (`self.CurrentState`) "NewEnumerator1")
      (set `self.CurrentState` "NewEnumerator2")
      (`/Game/Blueprints/ActorComponents/BaseSkill.StartRelease` (`self.kill_sk`)))))

(event `InputAction|Interact`
  (params (Key :type "Key Structure"))
  (bind _interactabletarget (`self.InteractableTarget`))
  ;[1 1 1] Interact
  (:`Pressed`
    (`/Engine/EditorBlueprintResources/StandardMacros.IsValid` _interactabletarget
      (:`Is Valid`
        (`self.Interact` _interactabletarget)))))

(event `self.ReceiveTick`
  (params (DeltaSeconds :type "Float (single-precision)")))

(event `self.ReceiveBeginPlay`)

(event `Key|Q`
  (params (Key :type "Key Structure")))

(event `OnFirstPerson`
  ;[1 1 1] Events for first and third camera
  (`SceneComponent.K2_SetRelativeLocation` (`self.Camera`) (.location (`SceneComponent.GetRelativeTransform` (`self.FirstCameraPlacement`))) false false)
  (`SceneComponent.K2_SetRelativeRotation` :`self` (`self.Camera`))
  (`PrimitiveComponent.SetCollisionEnabled` (`self.firstPersonInteractZone`) "QueryAndPhysics")
  (`PrimitiveComponent.SetCollisionEnabled` (`self.InteractTriggerZone`) "NoCollision")
  (set `self.nbOfInterectInZone` 0 :!label _label))

(event `InputAction|Sprint`
  (params (Key :type "Key Structure"))
  ;[1 1 1] Sprint System
  (:`Pressed`
    (if (`self.CanSprint`)
      (`self.OnStartSprinting` (`self.SprintMovementSpeed`))
      (set `self.IsSprinting` true)))
  (:`Released`
    (if (`self.IsSprinting`)
      (`self.OnStopSprinting` (`self.BaseMovementSpeed`))
      (set `self.IsSprinting` false))))

(event `OnThirdPerson`
  ;[1 1 1] Events for first and third camera
  (`SceneComponent.K2_SetRelativeLocation` (`self.Camera`) (.location (`SceneComponent.GetRelativeTransform` (`self.ThirdCameraPlacement`))) false false)
  (`SceneComponent.K2_SetRelativeRotation` (`self.Camera`) (struct :`Pitch` -20.0) false false)
  (`PrimitiveComponent.SetCollisionEnabled` (`self.InteractTriggerZone`) "QueryAndPhysics")
  (`PrimitiveComponent.SetCollisionEnabled` (`self.firstPersonInteractZone`) "NoCollision")
  (goto _label))

(event `OnStartSprinting`
  (params (SprintVelocity :type "Float (double-precision)"))
  ;[1 1 1] Sprint System
  (set `CharacterMovementComponent.MaxWalkSpeed` SprintVelocity (`self.CharacterMovement`)))

(event `OnStopSprinting`
  (params (BaseVelocity :type "Float (double-precision)"))
  ;[1 1 1] Sprint System
  (set `CharacterMovementComponent.MaxWalkSpeed` BaseVelocity (`self.CharacterMovement`)))

(event `InputAction|Crouch`
  (params (Key :type "Key Structure"))
  ;[1 1 1] Crouching System
  (:`Pressed`
    (`self.Crouch`))
  (:`Released`
    (`self.UnCrouch`)))

(event `InputAction|ToggleCamera`
  (params (Key :type "Key Structure"))
  ;[1 1 1] Trigger for first or third camera
  (:`Pressed`
    (if (`self.isFirstPerson`)
      (set `self.isFirstPerson` false)
      (`self.OnFirstPerson`)
      (else
        (set `self.isFirstPerson` true)
        (`self.OnThirdPerson`)))))

(event `self.InteractTriggerZone.OnComponentEndOverlap`
  (params (OverlappedComponent :type "PrimitiveComponent Object Reference") (OtherActor :type "Actor Object Reference") (OtherComp :type "PrimitiveComponent Object Reference") (OtherBodyIndex :type Integer)))

(event `self.firstPersonInteractZone.OnComponentBeginOverlap`
  (params (OverlappedComponent :type "PrimitiveComponent Object Reference") (OtherActor :type "Actor Object Reference") (OtherComp :type "PrimitiveComponent Object Reference") (OtherBodyIndex :type Integer) (bFromSweep :type Boolean) (SweepResult :type "HitResult Structure (by ref)"))
  (bind _returnvalue (+ (`self.nbOfInterectInZone`) 1))
  (set `self.nbOfInterectInZone` _returnvalue)
  (if (not (== _returnvalue 0))
    (set `self.containsInteractable` true)))

(event `self.firstPersonInteractZone.OnComponentEndOverlap`
  (params (OverlappedComponent :type "PrimitiveComponent Object Reference") (OtherActor :type "Actor Object Reference") (OtherComp :type "PrimitiveComponent Object Reference") (OtherBodyIndex :type Integer))
  (bind _interactabletarget (`self.InteractableTarget`))
  (bind _output_get (set `self.nbOfInterectInZone` (- (`self.nbOfInterectInZone`) 1)))
  (if (== _output_get 0)
    (set `self.containsInteractable` false)
    (`/Engine/EditorBlueprintResources/StandardMacros.IsValid` _interactabletarget
      (:`Is Valid`
        (`self.ToggleHighlight` _interactabletarget)
        (set `self.InteractableTarget` null)))))

(event `self.InteractTriggerZone.OnComponentBeginOverlap`
  (params (OverlappedComponent :type "PrimitiveComponent Object Reference") (OtherActor :type "Actor Object Reference") (OtherComp :type "PrimitiveComponent Object Reference") (OtherBodyIndex :type Integer) (bFromSweep :type Boolean) (SweepResult :type "HitResult Structure (by ref)")))

(fn `FindClosestTarget`
  (params (HitsArray :type "Array of HitResult Structure"))
  (returns (HitActor :type "Actor Object Reference"))
  (locals (DistanceArray :type "Array of Float (double-precision)"))
  (for _array_element HitsArray
    ;[1 1 1] Add all distances to DistanceArray
    (`KismetArrayLibrary.Array_Add` (`local.DistanceArray`) (`.Distance` (`GameplayStatics.BreakHitResult` _array_element))))
  (return (`.HitActor` (`GameplayStatics.BreakHitResult` (`|GetArrayItem` (`local.HitsArray`) (`KismetMathLibrary.MinOfFloatArray` (`local.DistanceArray`)))))))

(fn `Interact`
  (params (InteractableTarget :type "Actor Object Reference"))
  (bind _asbase_interactable (cast `BaseInteractable` InteractableTarget)
    (:`then`
      (`BaseInteractable.RespondInteract` _asbase_interactable self))
    (:`CastFailed`
      (`KismetSystemLibrary.PrintString` "Error in Interact "))))

(fn `MultipleToggleHighlight`
  (params (NewHits :type "Array of Actor Object Reference") (PreviousHits :type "Array of Actor Object Reference"))
  (for _array_element PreviousHits
    (`/Engine/EditorBlueprintResources/StandardMacros.IsValid` _array_element
      (:`Is Valid`
        (`self.ToggleHighlight` _array_element))
      (:`Is Not Valid`
        (`KismetSystemLibrary.PrintString` "no target to untoggle"))))
  (for _array_element_2 NewHits
    (`/Engine/EditorBlueprintResources/StandardMacros.IsValid` _array_element_2
      (:`Is Valid`
        (`self.ToggleHighlight` _array_element_2)))))

(fn `PrintoutAllHits`
  (params (Array :type "Array of HitResult Structure"))
  (for _array_element Array
    (bind (_bblockinghit _binitialoverlap _time _distance _location _impactpoint _normal _impactnormal _physmat _hitactor) (`GameplayStatics.BreakHitResult` _array_element))
    (`KismetSystemLibrary.PrintString` (`KismetStringLibrary.JoinStringArray` (`|MakeArray` (`KismetSystemLibrary.GetDisplayName` _hitactor) (`KismetStringLibrary.Conv_DoubleToString` _distance)) " | ") true false)))

(fn `ReturnToIdle`
  (set `self.CurrentState` "NewEnumerator0"))

(fn `ShperecastByMultiObject`
  (params (ObjectType :type "Array of EObjectTypeQuery Enum (by ref)" :default _))
  (returns (OutHits :type "Array of HitResult Structure") (ReturnValue :type Boolean))
  (bind _camera (`self.Camera`))
  (bind _returnvalue (`SceneComponent.K2_GetComponentLocation` _camera))
  ;[1 1 1] Cast a sphere in front of the camera
  (bind (_outhits _returnvalue_2) (`KismetSystemLibrary.SphereTraceMultiForObjects` _returnvalue (+ _returnvalue (* (`SceneComponent.GetForwardVector` _camera) (`self.DetectionRange`))) (`self.SpherecastRadius`) ObjectType))
  (return _outhits _returnvalue_2))

(fn `ShperecastBySingleObject`
  (params (ObjectType :type "Array of EObjectTypeQuery Enum" :default _) (Range :type "Float (double-precision)") (Radius :type "Float (double-precision)"))
  (returns (Target :type "HitResult Structure") (ReturnValue :type Boolean))
  (bind _camera (`self.Camera`))
  (bind _returnvalue (`SceneComponent.K2_GetComponentLocation` _camera))
  ;[1 1 1] Cast a sphere in front of the camera
  (bind (_outhit _returnvalue_2) (`KismetSystemLibrary.SphereTraceSingleForObjects` _returnvalue (+ _returnvalue (* (`SceneComponent.GetForwardVector` _camera) Range)) Radius ObjectType))
  (return _outhit _returnvalue_2))

(fn `TargetIndividual`
  (returns (Target :type "Actor Object Reference"))
  (locals (NewTarget :type "Actor Object Reference"))
  (bind _newtarget (`local.NewTarget`))
  (bind _enemytarget (`self.EnemyTarget`))
  (bind _enemytarget_2 (`self.EnemyTarget`))
  (bind (_outhits _returnvalue) (`self.ShperecastByMultiObject` (`|MakeArray` "ObjectTypeQuery7" :!type "EObjectTypeQuery Enum")))
  (if _returnvalue
    (bind _hitactor (`self.FindClosestTarget` _outhits))
    (set `local.NewTarget` _hitactor)
    ;[1 1 1] sets current target to new target, highlights it and removes highlight of the old target
    (`/Engine/EditorBlueprintResources/StandardMacros.IsValid` _enemytarget
      (:`Is Valid`
        (if (not (== _newtarget _enemytarget))
          (`self.ToggleHighlight` _enemytarget)
          (bind _output_get (set `self.EnemyTarget` _newtarget :!label _label))
          (`self.ToggleHighlight` _output_get)))
      (:`Is Not Valid`
        (goto _label)))
    (return _output_get)
    (else
      ;[1 1 1] No valid hit target - remove highlight from current target
      (`/Engine/EditorBlueprintResources/StandardMacros.IsValid` _enemytarget_2
        (:`Is Valid`
          (`self.ToggleHighlight` _enemytarget_2)
          (set `self.EnemyTarget` null)
          (return null))))))

(fn `TargetIndividualObject`
  (params (`Targeted Objects` :type "Array of EObjectTypeQuery Enum" :default _) (PreviousTarget :type "Actor Object Reference (by ref)") (Range :type "Float (double-precision)" :default 2000.0) (Radius :type "Float (double-precision)" :default 25.0))
  (returns (Target :type "Actor Object Reference"))
  (locals (NewTarget :type "Actor Object Reference"))
  (bind _previoustarget (`local.PreviousTarget`))
  (bind _newtarget (`local.NewTarget`))
  (bind _previoustarget_2 (`local.PreviousTarget`))
  (bind (_target _returnvalue) (`self.ShperecastBySingleObject` `Targeted Objects` Range Radius))
  (if _returnvalue
    (set `local.NewTarget` (`.HitActor` (`GameplayStatics.BreakHitResult` _target)))
    ;[1 1 1] sets current target to new target, highlights it and removes highlight of the old target
    (`/Engine/EditorBlueprintResources/StandardMacros.IsValid` _previoustarget_2
      (:`Is Valid`
        (if (not (== _newtarget _previoustarget_2))
          (`self.ToggleHighlight` _previoustarget_2)
          (`|VariableSetRef` (`local.PreviousTarget`) _newtarget :!label _label)
          (`self.ToggleHighlight` _newtarget)))
      (:`Is Not Valid`
        (goto _label)))
    (return _newtarget)
    (else
      ;[1 1 1] No valid hit target - remove highlight from current target
      (`/Engine/EditorBlueprintResources/StandardMacros.IsValid` _previoustarget
        (:`Is Valid`
          (`self.ToggleHighlight` _previoustarget)
          (`|VariableSetRef` _previoustarget)
          (return null))))))

(fn `TargetInteractable`
  (returns (Target :type "Actor Object Reference"))
  (locals (NewInteractable :type "Actor Object Reference"))
  (bind _interactabletarget (`self.InteractableTarget`))
  (bind _interactabletarget_2 (`self.InteractableTarget`))
  (bind _newinteractable (`local.NewInteractable`))
  (bind (_outhits _returnvalue) (`self.ShperecastByMultiObject` (`|MakeArray` "ObjectTypeQuery8" :!type "EObjectTypeQuery Enum")))
  (if _returnvalue
    (bind _hitactor (`self.FindClosestTarget` _outhits))
    (set `local.NewInteractable` _hitactor)
    ;[1 1 1] sets current target to new target, highlights it and removes highlight of the old target
    (`/Engine/EditorBlueprintResources/StandardMacros.IsValid` _interactabletarget_2
      (:`Is Valid`
        (if (not (== _newinteractable _interactabletarget_2))
          (`self.ToggleHighlight` _interactabletarget_2)
          (bind _output_get (set `self.InteractableTarget` _newinteractable :!label _label))
          (`self.ToggleHighlight` _output_get)))
      (:`Is Not Valid`
        (goto _label)))
    (return _output_get)
    (else
      ;[1 1 1] No valid hit target - remove highlight from current target
      (`/Engine/EditorBlueprintResources/StandardMacros.IsValid` _interactabletarget
        (:`Is Valid`
          (`self.ToggleHighlight` _interactabletarget)
          (set `self.InteractableTarget` null)
          (return null))))))

(fn `TargetMultipleObject`
  (params (MaxRange :type "Float (double-precision)") (MinimumRange :type "Float (double-precision)" :default 0.0) (SphereRadius :type "Float (double-precision)") (TargetedObject :type "Array of EObjectTypeQuery Enum" :default _) (previousTargets :type "Array of Actor Object Reference (by ref)") (NewParam :type Boolean))
  (locals (HitArray :type "Array of Actor Object Reference") (hasBeenDraw :type Boolean))
  (bind _camera (`self.Camera`))
  (bind _returnvalue (`SceneComponent.K2_GetComponentLocation` _camera))
  ;[1 1 1] This will find the first object the player is looking at and will get is location
  (bind (_outhit _returnvalue_2) (`KismetSystemLibrary.LineTraceSingleForObjects` _returnvalue (+ _returnvalue (* (`SceneComponent.GetForwardVector` _camera) MaxRange)) (`|MakeArray` "ObjectTypeQuery1" "ObjectTypeQuery7" "ObjectTypeQuery8" :!type "EObjectTypeQuery Enum")))
  ;[1 1 1] Check to make sure something was hit
  (if _returnvalue_2
    (bind (_bblockinghit _binitialoverlap _time _distance _location) (`GameplayStatics.BreakHitResult` _outhit))
    ;[1 1 1] cast a sphere at the location the player is looking at
    (bind (_outactors _returnvalue_3) (`KismetSystemLibrary.SphereOverlapActors` _location 300.0 (`local.TargetedObject`) null (`|MakeArray` self :!type "Actor Object Reference")))
    (if (`self.hasBeenDrawn`)
      (`SceneComponent.K2_SetWorldLocation` (`self.multipleTargetZone`) _location false false)
      (else
        (bind _returnvalue_4 (`AddComponent|NODE_AddStaticMeshComponent-1` :`bManualAttachment` true :`RelativeTransform` (`KismetMathLibrary.MakeTransform` _location (struct) (1.95 1.95 1.95))))
        (set `self.hasBeenDrawn` true)
        (`|VariableSetRef` (`self.multipleTargetZone`) _returnvalue_4)))
    (if _returnvalue_3
      (`|VariableSetRef` (`local.previousTargets`) _outactors)
      (else
        (`KismetSystemLibrary.PrintString` "No target found in the sphere")))
    (else
      (`KismetSystemLibrary.PrintString` "no target is near enough"))))

(fn `ToggleHighlight`
  (params (Actor :type "Actor Object Reference"))
  (returns (NewParam :type "Array of EObjectTypeQuery Enum"))
  (bind _returnvalue (`self.GetComponentByClass` Actor "/Script/Engine.StaticMeshComponent"))
  (`/Engine/EditorBlueprintResources/StandardMacros.IsValid` _returnvalue
    (:`Is Valid`
      (if (`PrimitiveComponent.bRenderCustomDepth` _returnvalue)
        (`PrimitiveComponent.SetRenderCustomDepth` _returnvalue false)
        (else
          (`PrimitiveComponent.SetRenderCustomDepth` _returnvalue true))))))

(fn `UserConstructionScript`)