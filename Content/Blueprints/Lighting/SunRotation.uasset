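; Sun actor that rotates continuously while time is passing, with a toggle function to start or stop it.
; On BeginPlay it registers itself in the StandardGameState's SunRotation variable and prints debug replication info.
; While IsTimePassing is set, Tick accumulates TimePassed and adds a fixed-rate pitch and roll rotation scaled by delta time.
; ToggleSunRotation sets that flag, and Tick prints a debug message while it is off.
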(event `self.ReceiveBeginPlay`
  ;[1 1 1] Attaching to gamemode on begin play
  (`KismetSystemLibrary.PrintString` (`KismetStringLibrary.Conv_BoolToString` (`self.bReplicates`)))
  (bind _asstandard_game_state (cast `/Game/Blueprints/GameModes/Standard/StandardGameState` (`GameplayStatics.GetGameState`))
    (:`then`
      (set `/Game/Blueprints/GameModes/Standard/StandardGameState.SunRotation` self _asstandard_game_state))
    (:`CastFailed`
      (`KismetSystemLibrary.PrintString` "failed to repliacted"))))

(event `self.ReceiveTick`
  (params (DeltaSeconds :type "Float (single-precision)"))
  ;[1 1 1] Sun rotation
  (if (`self.IsTimePassing`)
    (bind _output_get (set `self.TimePassed` (+ DeltaSeconds (`self.TimePassed`))))
    (`self.K2_SetActorRotation` (`KismetMathLibrary.ComposeRotators` (`self.K2_GetActorRotation`) (* (`KismetMathLibrary.MakeRotator` 12.728 12.728) DeltaSeconds)))
    (else
      (`KismetSystemLibrary.PrintString` "not passing" true true (struct :`G` 0.071122 :`B` 1.0 :`A` 1.0) 0.0))))

(fn `ToggleSunRotation`
  (params (`is rotating` :type Boolean))
  (set `self.IsTimePassing` `is rotating`))

(fn `UserConstructionScript`)