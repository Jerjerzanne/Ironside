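; Basic melee skill that gives the player character a close-range attack by spawning a hit collider.
; Execution spawns a scaled-down BaseMeleeAttack actor at the character's transform, attaches it with snap rules, and offsets it locally forward and to the side.
; It always returns true, leaving any hit handling to the spawned actor, and has no active event-graph logic.
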(fn `Execution`
  (returns (executed :type Boolean))
  (bind _playercharacter (`self.PlayerCharacter`))
  ;[1 1 1] Spawn attack collider
  (bind _returnvalue (`|SpawnActorFromClass` "/Game/Blueprints/MeleeAttacks/BaseMeleeAttack.BaseMeleeAttack_C" (`KismetMathLibrary.MakeTransform` (`Actor.K2_GetActorLocation` _playercharacter) (`Actor.K2_GetActorRotation` _playercharacter) (0.25 0.25 0.25)) "Undefined" "OverrideRootScale" null null))
  (`Actor.K2_AttachToActor` _returnvalue (`self.PlayerCharacter`) "None" "SnapToTarget" "SnapToTarget" "SnapToTarget" true)
  (`Actor.K2_AddActorLocalOffset` _returnvalue (100.0 70.0 0.0) false false)
  (return true))