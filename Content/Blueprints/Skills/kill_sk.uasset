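; Kill skill that destroys a single targeted actor and can chain into a finisher.
; While charging, Tick has the player character run individual targeting on one object type, passing in the current target.
; Execution saves the valid target's location, destroys the actor, then, if the finisher check passes, fires the current finisher there and starts its cooldown.
; It reports failure when no valid target exists.
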(event `self.ReceiveTick`
  (params (DeltaSeconds :type "Float (single-precision)"))
  (`parent.ReceiveTick` DeltaSeconds)
  (if (`self.Charging`)
    (`/Game/Blueprints/SimplePlayerCharacter.TargetIndividualObject` (`self.PlayerCharacter`) (`|MakeArray` "ObjectTypeQuery7" :!type "EObjectTypeQuery Enum") (`self.SingleTarget`) 2000.0 25.0)))

(fn `Execution`
  (returns (executed :type Boolean))
  (locals (`Finisher Position` :type "Vector Structure"))
  (bind _currentfinisher (`self.CurrentFinisher`))
  (bind _singletarget (`self.SingleTarget`))
  (`/Engine/EditorBlueprintResources/StandardMacros.IsValid` _singletarget
    (:`Is Valid`
      (set `local.Finisher Position` (`Actor.K2_GetActorLocation` _singletarget))
      (`Actor.K2_DestroyActor` _singletarget)
      (bind _usefinisher (`self.CheckFinisher`))
      (if _usefinisher
        (`self.Finisher` _currentfinisher (`local.Finisher Position`))
        (`self.SetCooldown` _currentfinisher))
      (return true))
    (:`Is Not Valid`
      (return false))))