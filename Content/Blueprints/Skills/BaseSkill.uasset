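; Base class for top-down player skills, handling charge, release and cooldown for the owning TopdownPlayerCharacter.
; Tick counts down charge and cooldown timers, pushing charge progress to the character and auto-releasing at full charge.
; Release clears the target zone and calls the overridable Execution, unless a required full charge is missing.
; Only successful execution starts cooldown and allows a delayed return to idle; finisher hooks are also provided.
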(event `self.ReceiveTick`
  (params (DeltaSeconds :type "Float (single-precision)"))
  (if (not (`self.CanCastSkill`))
    (`self.UpdateCD` DeltaSeconds))
  (if (`self.Charging`)
    (`self.UpdateCharge` DeltaSeconds)))

(event `self.ReceiveBeginPlay`
  (bind _astopdown_player_character (cast `/Game/Blueprints/TopdownPlayerCharacter` (`self.GetOwner`))
    (:`then`
      (set `self.PlayerCharacter` _astopdown_player_character))
    (:`CastFailed`
      (`KismetSystemLibrary.PrintString` "Skill has failed to attach player"))))

(fn `CheckFinisher`
  (returns (UseFinisher :type Boolean))
  (return (and (`KismetSystemLibrary.IsValid` (`self.CurrentFinisher`)) (`self.CanFinisher`))))

(fn `Execution`
  (returns (executed :type Boolean))
  (return false))

(fn `Finisher`
  (params (`Origin Finisher` :type "Vector Structure")))

(fn `OnFullyCharged`
  (`self.StartRelease` true))

(fn `RefreshCooldown`
  (set `self.CanCastSkill` true))

(fn `SetCooldown`
  (bind _maxcooldown (`self.MaxCooldown`))
  (set `self.CanCastSkill` false)
  (set `self.CooldownSeconds` _maxcooldown)
  (if (not (< 0.0 _maxcooldown))
    (`self.RefreshCooldown`)))

(fn `StartCharge`
  (bind _maxcasttime (`self.MaxCastTime`))
  (set `self.Charging` true)
  (if (< 0.0 _maxcasttime)
    (set `self.CastTimeSeconds` _maxcasttime)
    (else
      (`self.StartRelease` false))))

(fn `StartRelease`
  (params (FullyCharged :type Boolean))
  (bind _playercharacter (`self.PlayerCharacter`))
  (bind _releasetoidletime (`self.ReleaseToIdleTime`))
  (bind _playercharacter_2 (`self.PlayerCharacter`))
  (`/Game/Blueprints/TopdownPlayerCharacter.DestroyTargetZone` _playercharacter)
  (set `/Game/Blueprints/SimplePlayerCharacter.CurrentState` "NewEnumerator2" _playercharacter)
  (set `self.Charging` false)
  ;[1 1 1] Must this skill be fully charged?
  (if (`self.MustFullyCharge`)
    (if FullyCharged
      ;[1 1 1] Runs unique Execution function does not set the cooldown if it returns false
      (bind _executed (`self.Execution` :!label _label))
      (if _executed
        ;[1 1 1] Set cooldown of the skill
        (`self.SetCooldown`)
        (if (!= _releasetoidletime 0.0)
          (bind _returnvalue (`KismetSystemLibrary.K2_SetTimer` _playercharacter_2 "ReturnToIdle" _releasetoidletime))
          (set `self.ReleaseTimer` _returnvalue)
          (else
            (`/Game/Blueprints/BaseCharacter.ReturnToIdle` _playercharacter_2)))
        (else
          ;[1 1 1] dont set off cooldown
          (`/Game/Blueprints/SimplePlayerCharacter.ReturnToIdle` (`self.PlayerCharacter`) :!label _label_2)))
      (else
        (goto _label_2)))
    (else
      (goto _label))))

(fn `UpdateCD`
  (params (`time passed` :type "Float (double-precision)"))
  (bind _maxcooldown (`self.MaxCooldown`))
  (bind _output_get (set `self.CooldownSeconds` (- (`self.CooldownSeconds`) `time passed`)))
  (set `self.CooldownPercentage` (/ (- _maxcooldown _output_get) _maxcooldown))
  (if (<= _output_get 0.0)
    (`self.RefreshCooldown`)))

(fn `UpdateCharge`
  (params (TimePassed :type "Float (double-precision)"))
  (bind _maxcasttime (`self.MaxCastTime`))
  (bind _output_get (set `self.CastTimeSeconds` (- (`self.CastTimeSeconds`) TimePassed)))
  (bind _output_get_2 (set `self.CastTimePercentage` (/ (- _maxcasttime _output_get) _maxcasttime)))
  (set `/Game/Blueprints/SimplePlayerCharacter.ChargePercentage` _output_get_2 (`self.PlayerCharacter`))
  (if (<= _output_get 0.0)
    (`self.StartRelease` true)))