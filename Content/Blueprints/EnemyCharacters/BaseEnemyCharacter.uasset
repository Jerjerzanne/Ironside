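; BaseEnemyCharacter is an enemy character Blueprint that provides basic health and death handling.
; It fills current health to maximum on BeginPlay.
; Its TakeDamage event, noted as a damage interface override, subtracts incoming damage and calls Die at zero or below, which immediately destroys the actor.
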(event `self.ReceiveBeginPlay`
  ;[1 1 1] Set health to max
  (set `self.CurrentHealth` (`self.MaxHealth`)))

(event `self.TakeDamage`
  (params (Damage :type Integer))
  ;[1 1 1] Override the damage interface
  (bind _output_get (set `self.CurrentHealth` (- (`self.CurrentHealth`) Damage)))
  (if (<= _output_get 0)
    (`self.Die`)))

(event `self.Die`
  ;[1 1 1] Override the damage interface
  (`self.K2_DestroyActor`))

(fn `UserConstructionScript`)