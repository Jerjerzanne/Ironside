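; Water projectile actor that deals damage to what it overlaps.
; On overlap it ignores its instigator and passes ProjectileDamage and GameplayTags to TakeDamage on actors implementing DamageInterface.
; Any non-instigator overlap then calls OnProjectileEnd, whether or not damage was applied.
; BeginPlay and Tick are inactive, and the construction script only calls its parent.
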(event `self.ReceiveActorBeginOverlap`
  (params (OtherActor :type "Actor Object Reference"))
  (if (not (== OtherActor (`self.GetInstigator`)))
    (bind _asdamage_interface (cast `/Game/Blueprints/Interfaces/DamageInterface` OtherActor)
      (:`then`
        (`/Game/Blueprints/Interfaces/DamageInterface.TakeDamage` _asdamage_interface (`self.ProjectileDamage`) (`self.GameplayTags`))
        (`self.OnProjectileEnd`))
      (:`CastFailed`
        (`self.OnProjectileEnd`)))))

(fn `UserConstructionScript`
  (`parent.UserConstructionScript`))