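; Base projectile Blueprint that destroys itself through OnProjectileEnd when its collision component registers a hit.
; Helper functions test whether travel from a start point has reached max range and treat anything other than the Instigator as an enemy.
; GetEndLocation flattens the forward vector to XY, scales it by range and keeps the actor's Z, without adding the actor's XY position.
; No movement, damage or calls to these helpers appear here.
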(event `self.Collision.OnComponentHit`
  (params (HitComponent :type "PrimitiveComponent Object Reference") (OtherActor :type "Actor Object Reference") (OtherComp :type "PrimitiveComponent Object Reference") (NormalImpulse :type "Vector Structure") (Hit :type "HitResult Structure (by ref)"))
  ;[1 1 1] Delete the projectile if it hits a wall
  (`self.OnProjectileEnd`))

(fn `getEndLocation`
  (params (Range :type "Float (double-precision)"))
  (returns (EndLocation :type "Vector Structure"))
  ;[1 1 1] Return the end location of the projectile
  (return (`KismetMathLibrary.Conv_Vector2DToVector` (* (`KismetMathLibrary.Conv_VectorToVector2D` (`self.GetActorForwardVector`)) Range) (.z (`self.K2_GetActorLocation`)))))

(fn `HasReachedMaxRange`
  (params (CurrentLocation :type "Vector Structure") (StartingLocation :type "Vector Structure") (MaxDistance :type "Float (double-precision)"))
  (returns (isAtMaxDistance :type Boolean))
  ;[0.6609 0.7316 1] Return if the projectile has reached his max distance
  (return (>= (`KismetMathLibrary.VSize` (- CurrentLocation StartingLocation)) MaxDistance)))

(fn `is Target an Enemy`
  (params (`Entity to Check` :type "Actor Object Reference"))
  (returns (isEnemy :type Boolean))
  ;[0.3297 0.3626 1] This function return whether or not the target is an enemy of the owner of the projectile
  (return (!= `Entity to Check` (`self.GetInstigator`))))

(fn `OnProjectileEnd`
  (`self.K2_DestroyActor`))

(fn `UserConstructionScript`)