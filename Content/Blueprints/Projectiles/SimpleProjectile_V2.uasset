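; A GAS projectile that flies a curved path out to the distance of the instigator's mouse position and damages enemies it overlaps.
; Construction derives the range from that position, then a Timeline moves the actor forward while a float curve offsets it sideways.
; Enemy overlap applies set-by-caller damage and extra effects, then ends the projectile, as does exceeding range.
; Homing logic is unconnected, and debug prints remain.
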(event `self.ReceiveBeginPlay`
  (`self.Move along the curve`))

(event `self.ReceiveActorBeginOverlap`
  (params (OtherActor :type "Actor Object Reference"))
  (bind _returnvalue (`AbilitySystemBlueprintLibrary.GetAbilitySystemComponent` OtherActor))
  (bind _asc_basefireprojectile (`self.ASC_BaseFireProjectile`))
  (bind _isenemy (`self.is Target an Enemy` OtherActor))
  (if _isenemy
    (bind _result (`/Engine/EditorBlueprintResources/StandardMacros.NegateInt` (`self.ProjectileDamage`))
      (:`  `
        (bind _returnvalue_2 (`AbilitySystemBlueprintLibrary.AssignTagSetByCallerMagnitude` (`AbilitySystemComponent.MakeOutgoingSpec` :`self` (`self.ASC_BaseFireProjectile`) :`GameplayEffectClass` "/Game/GameplayAbilities/Effects/GE_Damage.GE_Damage_C" :`Level` 1.0) (struct :`TagName` "Gameplay.Damage") (`KismetMathLibrary.Conv_IntToDouble` _result)))
        (`AbilitySystemComponent.BP_ApplyGameplayEffectSpecToTarget` _asc_basefireprojectile _returnvalue_2 _returnvalue)
        (for _array_element (`self.ProjectileEffects`)
          (`AbilitySystemComponent.BP_ApplyGameplayEffectToTarget` :`self` _asc_basefireprojectile :`GameplayEffectClass` _array_element :`Target` _returnvalue :`Level` 1.0))
        (`self.OnProjectileEnd`)))))

(event `self.ReceiveTick`
  (params (DeltaSeconds :type "Float (single-precision)"))
  ;[1 1 1] Checking if Projectile has reach max Distance, if true, destroy the projectile
  (bind _isatmaxdistance (`self.HasReachedMaxRange` (`self.K2_GetActorLocation`) (`self.StartingLocation`) (`self.MaxRange`)))
  (if _isatmaxdistance
    (`self.OnProjectileEnd`)))

(event `Move along the curve`
  (bind (_direction _alpha) (`Timeline|Timeline_0`)
    (:`Update`
      (bind _returnvalue (+ (* (* (`self.GetActorRightVector`) (`CurveFloat.GetFloatValue` (`self.CurveFloat`) _alpha)) (`self.DeviationNorm`)) (* (* (`self.GetActorForwardVector`) _alpha) (`self.MaxRange`)) (`self.StartingLocation`)))
      (`self.K2_SetActorLocation` _returnvalue)
      (`KismetSystemLibrary.PrintString` (`KismetStringLibrary.Concat_StrStr` "Projectile Locations:" (`KismetStringLibrary.Conv_VectorToString` _returnvalue)) true true (struct :`R` 0.064395 :`G` 1.0 :`B` 0.017018 :`A` 1.0) 0.0))))

(fn `UserConstructionScript`
  (`parent.UserConstructionScript`)
  (bind _output_get (set `self.StartingLocation` (`self.K2_GetActorLocation`)))
  (bind _asbase_character (cast `/Game/Blueprints/Characters/BaseCharacter` (`self.GetInstigator`)))
  (bind _mouseposition (`/Game/Blueprints/Characters/BaseCharacter.MousePosition` _asbase_character))
  (bind _output_get_2 (set `self.MouseTargetLocation` _mouseposition))
  (`KismetSystemLibrary.PrintString` (`KismetStringLibrary.Conv_VectorToString` _output_get_2) true true (struct :`R` 1.0 :`G` 0.078125 :`B` 0.270625 :`A` 1.0))
  (bind _output_get_3 (set `self.MaxRange` (`KismetMathLibrary.VSize` (- _mouseposition (`KismetMathLibrary.MakeVector` (.x _output_get) (.y _output_get))))))
  (`KismetSystemLibrary.PrintString` (`KismetStringLibrary.Conv_DoubleToString` _output_get_3) true true (struct :`R` 1.0 :`G` 0.740545 :`A` 1.0) 5.0))