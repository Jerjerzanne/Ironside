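; Player character Blueprint that lets the player toggle its camera between first-person and third-person views.
; Pressing P flips the IsFirstPerson flag and calls the matching custom event.
; Each event snaps the Camera to the relative location of a first- or third-person placement component and sets a fixed rotation, level for first person and pitched down for third.
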(event `OnFirstPerson`
  ;[1 1 1] Events for first and third camera
  (`SceneComponent.K2_SetRelativeLocation` (`self.Camera`) (.location (`SceneComponent.GetRelativeTransform` (`self.FirstCameraPlacement`))) false false)
  (`SceneComponent.K2_SetRelativeRotation` :`self` (`self.Camera`)))

(event `OnThirdPerson`
  ;[1 1 1] Events for first and third camera
  (`SceneComponent.K2_SetRelativeLocation` (`self.Camera`) (.location (`SceneComponent.GetRelativeTransform` (`self.ThirdCameraPlacement`))) false false)
  (`SceneComponent.K2_SetRelativeRotation` (`self.Camera`) (struct :`Pitch` -20.0) false false))

(event `Key|P`
  (params (Key :type "Key Structure"))
  ;[1 1 1] Trigger for first or third camera
  (:`Pressed`
    (if (`self.isFirstPerson`)
      (set `self.isFirstPerson` false)
      (`self.OnThirdPerson`)
      (else
        (set `self.isFirstPerson` true)
        (`self.OnFirstPerson`)))))

(fn `UserConstructionScript`)