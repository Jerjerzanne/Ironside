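; Simple player projectile actor that flies in a straight line and damages what it touches.
; Each tick it moves along the normalized Direction at ProjectileSpeed by setting its location without sweep.
; On actor overlap it passes ProjectileDamage to TakeDamage on targets implementing DamageInterface, then destroys itself whether or not the cast succeeds.
; A Hit event also destroys it, without applying damage.
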(event `self.ReceiveTick`
  (params (DeltaSeconds :type "Float (single-precision)"))
  ;[1 1 1] Translation
  (`self.K2_SetActorLocation` (+ (* (`KismetMathLibrary.Normal` (`self.Direction`)) (* DeltaSeconds (`self.ProjectileSpeed`))) (`self.K2_GetActorLocation`))))

(event `self.ReceiveActorBeginOverlap`
  (params (OtherActor :type "Actor Object Reference"))
  (bind _asdamage_interface (cast `/Game/Interfaces/DamageInterface` OtherActor)
    (:`then`
      (`/Game/Blueprints/EnemyCharacters/BaseEnemyCharacter.TakeDamage` _asdamage_interface (`self.ProjectileDamage`)))
    (:`CastFailed`
      _))
  (`self.K2_DestroyActor` :!label _label))

(event `self.ReceiveHit`
  (params (MyComp :type "PrimitiveComponent Object Reference") (Other :type "Actor Object Reference") (OtherComp :type "PrimitiveComponent Object Reference") (bSelfMoved :type Boolean) (HitLocation :type "Vector Structure") (HitNormal :type "Vector Structure") (NormalImpulse :type "Vector Structure") (Hit :type "HitResult Structure (by ref)"))
  (goto _label))

(fn `UserConstructionScript`)