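; Player character with switchable first/third-person camera, sprint, crouch, health and key-mapped skills.
; Camera-specific trigger zones exist, but only first-person overlaps count interactables, gating a per-tick sphere trace that highlights the target via custom depth for Interact.
; Skill input starts charging, releases on repeat press, or queues a finisher mid-charge.
; Also holds multi-target, FOV and target-zone helpers, plus test mouse bindings for healing and damage.
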(event `self.firstPersonInteractZone.OnComponentBeginOverlap`
  (params (OverlappedComponent :type "PrimitiveComponent Object Reference") (OtherActor :type "Actor Object Reference") (OtherComp :type "PrimitiveComponent Object Reference") (OtherBodyIndex :type Integer) (bFromSweep :type Boolean) (SweepResult :type "HitResult Structure (by ref)"))
  (bind _returnvalue (+ (`self.nbOfInterectInZone`) 1))
  ;[1 1 1] Interactable Trigger Zone
  (set `self.nbOfInterectInZone` _returnvalue)
  (if (not (== _returnvalue 0))
    (set `self.containsInteractable` true)))

(event `InputAction|Interact`
  (params (Key :type "Key Structure"))
  (bind _interactabletarget (`self.InteractableTarget`))
  ;[1 1 1] Interact
  (:`Pressed`
    (`/Engine/EditorBlueprintResources/StandardMacros.IsValid` _interactabletarget
      (:`Is Valid`
        (`self.Interact` _interactabletarget)))))

(event `self.firstPersonInteractZone.OnComponentEndOverlap`
  (params (OverlappedComponent :type "PrimitiveComponent Object Reference") (OtherActor :type "Actor Object Reference") (OtherComp :type "PrimitiveComponent Object Reference") (OtherBodyIndex :type Integer))
  (bind _interactabletarget (`self.InteractableTarget`))
  ;[1 1 1] Interactable Trigger Zone
  (bind _output_get (set `self.nbOfInterectInZone` (- (`self.nbOfInterectInZone`) 1)))
  (if (== _output_get 0)
    (set `self.containsInteractable` false)
    (`/Engine/EditorBlueprintResources/StandardMacros.IsValid` _interactabletarget
      (:`Is Valid`
        (`self.ToggleHighlight` _interactabletarget)
        (set `self.InteractableTarget` null)))))

(event `self.InteractTriggerZone.OnComponentBeginOverlap`
  (params (OverlappedComponent :type "PrimitiveComponent Object Reference") (OtherActor :type "Actor Object Reference") (OtherComp :type "PrimitiveComponent Object Reference") (OtherBodyIndex :type Integer) (bFromSweep :type Boolean) (SweepResult :type "HitResult Structure (by ref)"))
  ;[1 1 1] Interactable Trigger Zone
)

(event `self.InteractTriggerZone.OnComponentEndOverlap`
  (params (OverlappedComponent :type "PrimitiveComponent Object Reference") (OtherActor :type "Actor Object Reference") (OtherComp :type "PrimitiveComponent Object Reference") (OtherBodyIndex :type Integer))
  ;[1 1 1] Interactable Trigger Zone
)

(event `self.ReceiveTick`
  (params (DeltaSeconds :type "Float (single-precision)"))
  ;[1 1 1] Triggers highlight on the interact
  (if (`self.containsInteractable`)
    (`self.TargetIndividualObject` (`|MakeArray` "ObjectTypeQuery8" :!type "EObjectTypeQuery Enum") (`self.InteractableTarget`) (`self.DetectionRange`) 3.0)))

(event `InputAction|Skill1`
  (params (Key :type "Key Structure"))
  ;[1 1 1] Skill input management
  (:`Pressed`
    (`self.ProcessSkillInput` Key)))

(event `InputAction|Skill2`
  (params (Key :type "Key Structure"))
  ;[1 1 1] Skill input management
  (:`Pressed`
    (`self.ProcessSkillInput` Key)))

(event `InputAction|Skill3`
  (params (Key :type "Key Structure"))
  ;[1 1 1] Skill input management
  (:`Pressed`
    (`self.ProcessSkillInput` Key)))

(event `InputAction|Skill4`
  (params (Key :type "Key Structure"))
  ;[1 1 1] Skill input management
  (:`Pressed`
    (`self.ProcessSkillInput` Key)))

(event `self.ReceiveBeginPlay`
  ;[1 1 1] BeginPlay
  (`self.SetHealthToMax`)
  (bind _output_get (set `self.SkillMap` (`|MakeMap` "E" null "Q" null "R" (`self.heal_sk`) "T" (`self.basicProjectile_sk`) :!type "Key Structure" :!valuetype "/Game/Blueprints/Skills/BaseSkill Object Reference")))
  (bind _values (`BlueprintMapLibrary.Map_Values` _output_get))
  (set `self.SkillInventory` _values))

(event `OnFirstPerson`
  ;[1 1 1] Events for first and third camera
  (`SceneComponent.K2_SetRelativeLocation` (`self.Camera`) (.location (`SceneComponent.GetRelativeTransform` (`self.FirstCameraPlacement`))) false false)
  (`SceneComponent.K2_SetRelativeRotation` :`self` (`self.Camera`))
  (`PrimitiveComponent.SetCollisionEnabled` (`self.firstPersonInteractZone`) "QueryAndPhysics")
  (`PrimitiveComponent.SetCollisionEnabled` (`self.InteractTriggerZone`) "NoCollision")
  (set `self.nbOfInterectInZone` 0 :!label _label))

(event `InputAction|Sprint`
  (params (Key :type "Key Structure"))
  ;[0.9529 0.7232 1] Sprint System
  (:`Pressed`
    (if (`self.CanSprint`)
      (`self.OnStartSprinting` (`self.SprintMovementSpeed`))
      (set `self.IsSprinting` true)))
  (:`Released`
    (if (`self.IsSprinting`)
      (`self.OnStopSprinting` (`self.BaseMovementSpeed`))
      (set `self.IsSprinting` false))))

(event `OnStartSprinting`
  (params (SprintVelocity :type "Float (double-precision)"))
  ;[0.9529 0.7232 1] Sprint System
  (set `CharacterMovementComponent.MaxWalkSpeed` SprintVelocity (`self.CharacterMovement`)))

(event `OnThirdPerson`
  ;[1 1 1] Events for first and third camera
  (`SceneComponent.K2_SetRelativeLocation` (`self.Camera`) (.location (`SceneComponent.GetRelativeTransform` (`self.ThirdCameraPlacement`))) false false)
  (`SceneComponent.K2_SetRelativeRotation` (`self.Camera`) (struct :`Pitch` -20.0) false false)
  (`PrimitiveComponent.SetCollisionEnabled` (`self.InteractTriggerZone`) "QueryAndPhysics")
  (`PrimitiveComponent.SetCollisionEnabled` (`self.firstPersonInteractZone`) "NoCollision")
  (goto _label))

(event `OnStopSprinting`
  (params (BaseVelocity :type "Float (double-precision)"))
  ;[0.9529 0.7232 1] Sprint System
  (set `CharacterMovementComponent.MaxWalkSpeed` BaseVelocity (`self.CharacterMovement`)))

(event `Key|LeftMouseButton`
  (params (Key :type "Key Structure"))
  ;[1 1 1] Test functions to tweak HP values
  (:`Pressed`
    (`self.Heal` 10)))

(event `Key|RightMouseButton`
  (params (Key :type "Key Structure"))
  ;[1 1 1] Test functions to tweak HP values
  (:`Pressed`
    (`self.TakeDamage` 10)))

(event `InputAction|Crouch`
  (params (Key :type "Key Structure"))
  ;[0.3864 0.2961 0.4072] Crouching System
  (:`Pressed`
    (`self.Crouch`))
  (:`Released`
    (`self.UnCrouch`)))

(event `InputAction|ToggleCamera`
  (params (Key :type "Key Structure"))
  ;[1 1 1] Trigger for first or third camera
  (:`Pressed`
    (if (`self.isFirstPerson`)
      (set `self.isFirstPerson` false)
      (`self.OnThirdPerson`)
      (else
        (set `self.isFirstPerson` true)
        (`self.OnFirstPerson`)))))

(fn `AddActorComponentToPlayer`
  (params (ObjectToAdd :type "ActorComponent Object Reference")))

(fn `AutoTargetObject`
  (params (PreviousTargets :type "Array of Actor Object Reference (by ref)") (range :type "Float (double-precision)" :default 500.0) (TargetedObject :type "Array of EObjectTypeQuery Enum" :default _) (RequiredNbOfHit :type Integer :default 1))
  (locals (InFOV :type "Array of Actor Object Reference"))
  (bind (_outactors _returnvalue) (`KismetSystemLibrary.SphereOverlapActors` (`self.K2_GetActorLocation` self) range TargetedObject null (`|MakeArray` self :!type "Actor Object Reference")))
  (if _returnvalue
    (for _array_element _outactors
      (bind _isactorinfov (`self.IsActorInFOV` _array_element))
      (if _isactorinfov
        (`KismetArrayLibrary.Array_Add` (`local.InFOV`) _array_element)))))

(fn `DestroyTargetZone`
  (bind _multipletargetzone (`self.multipleTargetZone`))
  (`/Engine/EditorBlueprintResources/StandardMacros.IsValid` _multipletargetzone
    (:`Is Valid`
      (`ActorComponent.K2_DestroyComponent` _multipletargetzone)
      (set `self.multipleTargetZone` null)
      (set `self.hasBeenDrawn` false))))

(fn `DrawTargetZone`
  (params (arguments :type "Map of String to Integer") (material :type String) (targetZone :type String) (location :type "Vector Structure"))
  (bind _multipletargetzone (`self.multipleTargetZone`))
  (bind (_value _returnvalue) (`BlueprintMapLibrary.Map_Find` (`local.arguments`) "radius"))
  (bind _returnvalue_2 (/ (`KismetMathLibrary.Conv_IntToDouble` _value) 153.850006))
  (switch `string` targetZone
    (:`sphere`
      (if (`self.hasBeenDrawn`)
        (`/Engine/EditorBlueprintResources/StandardMacros.IsValid` _multipletargetzone
          (:`Is Valid`
            (`SceneComponent.K2_SetWorldLocation` _multipletargetzone (`local.location`) false false)))
        (elif _returnvalue
          (bind _returnvalue_3 (`AddComponent|NODE_AddStaticMeshComponent-2` :`RelativeTransform` (`KismetMathLibrary.MakeTransform` (`local.location`) (struct) (`KismetMathLibrary.MakeVector` _returnvalue_2 _returnvalue_2 _returnvalue_2))))
          (set `self.multipleTargetZone` _returnvalue_3)
          (set `self.hasBeenDrawn` true))))))

(fn `FindAngleBetweenVectors`
  (params (A :type "Vector Structure") (B :type "Vector Structure"))
  (returns (Angle :type "Float (double-precision)"))
  (bind _returnvalue (`KismetMathLibrary.Normal` A))
  (bind _returnvalue_2 (`KismetMathLibrary.Normal` B))
  (`KismetSystemLibrary.PrintString` (`KismetStringLibrary.Conv_VectorToString` _returnvalue))
  (`KismetSystemLibrary.PrintString` (`KismetStringLibrary.Conv_VectorToString` _returnvalue_2))
  (return (`KismetMathLibrary.DegAcos` (`KismetMathLibrary.Dot_VectorVector` _returnvalue _returnvalue_2))))

(fn `FindClosestTarget`
  (params (HitsArray :type "Array of HitResult Structure"))
  (returns (HitActor :type "Actor Object Reference"))
  (locals (DistanceArray :type "Array of Float (double-precision)"))
  (for _array_element HitsArray
    ;[1 1 1] Add all distances to DistanceArray
    (`KismetArrayLibrary.Array_Add` (`local.DistanceArray`) (`.Distance` (`GameplayStatics.BreakHitResult` _array_element))))
  (return (`.HitActor` (`GameplayStatics.BreakHitResult` (`|GetArrayItem` (`local.HitsArray`) (`KismetMathLibrary.MinOfFloatArray` (`local.DistanceArray`)))))))

(fn `Heal`
  (params (`Heal amount` :type Integer))
  (bind _output_get (set `self.CurrentHealth` (+ (`self.CurrentHealth`) `Heal amount`)))
  (if (> _output_get (`self.MaxHealth`))
    (`self.SetHealthToMax`)))

(fn `Interact`
  (params (InteractableTarget :type "Actor Object Reference"))
  (bind _asbase_interactable (cast `BaseInteractable` InteractableTarget)
    (:`then`
      (`BaseInteractable.RespondInteract` _asbase_interactable self))
    (:`CastFailed`
      (`KismetSystemLibrary.PrintString` "Error in Interact "))))

(fn `IsActorInFOV`
  (params (actor :type "Actor Object Reference"))
  (returns (isActorInFOV :type Boolean))
  (bind _angle (`self.FindAngleBetweenVectors` (`SceneComponent.GetForwardVector` (`self.Camera`)) (`KismetMathLibrary.InverseTransformLocation` (`KismetMathLibrary.Conv_VectorToTransform` (`SceneComponent.K2_GetComponentLocation` (`self.CapsuleComponent`))) (`self.K2_GetActorLocation` actor))))
  (return (< _angle 46.0)))

(fn `MultipleToggleHighlight`
  (params (NewHits :type "Array of Actor Object Reference") (PreviousHits :type "Array of Actor Object Reference"))
  (for _array_element PreviousHits
    (`/Engine/EditorBlueprintResources/StandardMacros.IsValid` _array_element
      (:`Is Valid`
        (`self.ToggleHighlight` _array_element))
      (:`Is Not Valid`
        (`KismetSystemLibrary.PrintString` "no target to untoggle"))))
  (for _array_element_2 NewHits
    (`/Engine/EditorBlueprintResources/StandardMacros.IsValid` _array_element_2
      (:`Is Valid`
        (`self.ToggleHighlight` _array_element_2)))))

(fn `PrintoutAllHits`
  (params (Array :type "Array of HitResult Structure"))
  (for _array_element Array
    (bind (_bblockinghit _binitialoverlap _time _distance _location _impactpoint _normal _impactnormal _physmat _hitactor) (`GameplayStatics.BreakHitResult` _array_element))
    (`KismetSystemLibrary.PrintString` (`KismetStringLibrary.JoinStringArray` (`|MakeArray` (`KismetSystemLibrary.GetDisplayName` _hitactor) (`KismetStringLibrary.Conv_DoubleToString` _distance)) " | ") true false)))

(fn `ProcessSkillInput`
  (params (Key :type "Key Structure (by ref)"))
  (bind _currentskill (`self.CurrentSkill`))
  (bind (_value _returnvalue) (`BlueprintMapLibrary.Map_Find` (`self.SkillMap`) Key))
  ;[1 1 1] is your input mapped to a skill?
  (if (and (`KismetSystemLibrary.IsValid` _value) _returnvalue)
    (`/Engine/EditorBlueprintResources/StandardMacros.IsValid` _currentskill
      (:`Is Valid`
        (if (== _value _currentskill)
          (`self.TryRelease` _value)
          (elif (and (`/Game/Blueprints/Skills/BaseSkill.IsFinisher` _value) (`/Game/Blueprints/Skills/BaseSkill.CanFinisher` _currentskill) (`/Game/Blueprints/Skills/BaseSkill.Charging` _currentskill))
            (set `/Game/Blueprints/Skills/BaseSkill.CurrentFinisher` _value _currentskill))))
      (:`Is Not Valid`
        (`self.TryCharging` _value)))
    (else
      (`KismetSystemLibrary.PrintString` "invalid spell"))))

(fn `ResetChargeBar`
  (set `self.CurrentSkill` null)
  (set `self.ChargePercentage` 0.0))

(fn `ShperecastByMultiObject`
  (params (ObjectType :type "Array of EObjectTypeQuery Enum (by ref)" :default _))
  (returns (OutHits :type "Array of HitResult Structure") (ReturnValue :type Boolean))
  (bind _camera (`self.Camera`))
  (bind _returnvalue (`SceneComponent.K2_GetComponentLocation` _camera))
  ;[1 1 1] Cast a sphere in front of the camera
  (bind (_outhits _returnvalue_2) (`KismetSystemLibrary.SphereTraceMultiForObjects` _returnvalue (+ _returnvalue (* (`SceneComponent.GetForwardVector` _camera) (`self.DetectionRange`))) (`self.SpherecastRadius`) ObjectType))
  (return _outhits _returnvalue_2))

(fn `ShperecastBySingleObject`
  (params (ObjectType :type "Array of EObjectTypeQuery Enum" :default _) (Range :type "Float (double-precision)") (Radius :type "Float (double-precision)"))
  (returns (Target :type "HitResult Structure") (ReturnValue :type Boolean))
  (bind _camera (`self.Camera`))
  (bind _returnvalue (`SceneComponent.K2_GetComponentLocation` _camera))
  ;[1 1 1] Cast a sphere in front of the camera
  (bind (_outhit _returnvalue_2) (`KismetSystemLibrary.SphereTraceSingleForObjects` _returnvalue (+ _returnvalue (* (`SceneComponent.GetForwardVector` _camera) Range)) Radius ObjectType))
  (return _outhit _returnvalue_2))

(fn `TargetIndividualObject`
  (params (`Targeted Objects` :type "Array of EObjectTypeQuery Enum" :default _) (PreviousTarget :type "Actor Object Reference (by ref)") (Range :type "Float (double-precision)" :default 2000.0) (Radius :type "Float (double-precision)" :default 25.0))
  (returns (Target :type "Actor Object Reference"))
  (locals (NewTarget :type "Actor Object Reference"))
  (bind _previoustarget (`local.PreviousTarget`))
  (bind _newtarget (`local.NewTarget`))
  (bind _previoustarget_2 (`local.PreviousTarget`))
  (bind (_target _returnvalue) (`self.ShperecastBySingleObject` `Targeted Objects` Range Radius))
  (if _returnvalue
    (set `local.NewTarget` (`.HitActor` (`GameplayStatics.BreakHitResult` _target)))
    ;[1 1 1] sets current target to new target, highlights it and removes highlight of the old target
    (`/Engine/EditorBlueprintResources/StandardMacros.IsValid` _previoustarget_2
      (:`Is Valid`
        (if (not (== _newtarget _previoustarget_2))
          (`self.ToggleHighlight` _previoustarget_2)
          (`|VariableSetRef` (`local.PreviousTarget`) _newtarget :!label _label)
          (`self.ToggleHighlight` _newtarget)))
      (:`Is Not Valid`
        (goto _label)))
    (return _newtarget)
    (else
      ;[1 1 1] No valid hit target - remove highlight from current target
      (`/Engine/EditorBlueprintResources/StandardMacros.IsValid` _previoustarget
        (:`Is Valid`
          (`self.ToggleHighlight` _previoustarget)
          (`|VariableSetRef` _previoustarget)
          (return null))))))

(fn `TargetMultipleObject`
  (params (MaxRange :type "Float (double-precision)") (MinimumRange :type "Float (double-precision)" :default 0.0) (SphereRadius :type "Float (double-precision)") (TargetedObject :type "Array of EObjectTypeQuery Enum" :default _) (previousTargets :type "Array of Actor Object Reference (by ref)") (NewParam :type Boolean))
  (returns (sphereLocation :type "Vector Structure"))
  (locals (HitArray :type "Array of Actor Object Reference") (hasBeenDraw :type Boolean) (lineTraceLocation :type "Vector Structure") (NewLocalVar_0 :type "Array of Actor Object Reference"))
  (bind _camera (`self.Camera`))
  (bind _returnvalue (`SceneComponent.K2_GetComponentLocation` _camera))
  ;[1 1 1] This will find the first object the player is looking at and will get is location
  (bind (_outhit _returnvalue_2) (`KismetSystemLibrary.LineTraceSingleForObjects` _returnvalue (+ _returnvalue (* (`SceneComponent.GetForwardVector` _camera) MaxRange)) (`|MakeArray` "ObjectTypeQuery1" "ObjectTypeQuery7" "ObjectTypeQuery8" :!type "EObjectTypeQuery Enum")))
  ;[1 1 1] Check to make sure something was hit
  (if _returnvalue_2
    (bind (_bblockinghit _binitialoverlap _time _distance _location) (`GameplayStatics.BreakHitResult` _outhit))
    ;[1 1 1] cast a sphere at the location the player is looking at
    (set `local.lineTraceLocation` _location)
    (bind (_outactors _returnvalue_3) (`KismetSystemLibrary.SphereOverlapActors` _location 300.0 (`local.TargetedObject`) null (`|MakeArray` self :!type "Actor Object Reference")))
    (if _returnvalue_3
      (`|VariableSetRef` (`local.previousTargets`) _outactors)
      (else
        (`KismetArrayLibrary.Array_Clear` (`local.previousTargets`))))
    (return (`local.lineTraceLocation`))
    (else
      (`KismetSystemLibrary.PrintString` "no target is near enough"))))

(fn `ToggleHighlight`
  (params (Actor :type "Actor Object Reference"))
  (returns (NewParam :type "Array of EObjectTypeQuery Enum"))
  (bind _returnvalue (`self.GetComponentByClass` Actor "/Script/Engine.StaticMeshComponent"))
  (`/Engine/EditorBlueprintResources/StandardMacros.IsValid` _returnvalue
    (:`Is Valid`
      (if (`PrimitiveComponent.bRenderCustomDepth` _returnvalue)
        (`PrimitiveComponent.SetRenderCustomDepth` _returnvalue false)
        (else
          (`PrimitiveComponent.SetRenderCustomDepth` _returnvalue true))))))

(fn `UserConstructionScript`)