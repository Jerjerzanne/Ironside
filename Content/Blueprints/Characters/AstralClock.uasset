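; AstralClock is a game-time controller that uses the Gameplay Ability System to start, stop and resume time for players.
; Each function loops over the Players array and casts each controlled pawn to PlayerCharacter.
; StartClock applies the GE_Day effect and StopClock applies GE_StopTime through the clock's AbilitySystem.
; ResumeClock removes effects tagged Gameplay.Time.Stop and prints the removal count as debug output.
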(fn `ResumeClock`
  (for _array_element (`self.Players`)
    (bind _asplayer_character (cast `/Game/Blueprints/Characters/PlayerCharacter` (`Controller.K2_GetPawn` _array_element))
      (:`then`
        (bind _returnvalue (`AbilitySystemComponent.RemoveActiveEffectsWithAppliedTags` (`AbilitySystemBlueprintLibrary.GetAbilitySystemComponent` _asplayer_character) (struct :`GameplayTags` (struct :`(TagName` "Gameplay.Time.Stop")))))
        (`KismetSystemLibrary.PrintString` (`KismetStringLibrary.Conv_IntToString` _returnvalue) true true (struct :`R` 1.0 :`G` 0.19407 :`B` 0.555345 :`A` 1.0)))
      (:`CastFailed`
        (`KismetSystemLibrary.PrintString` "Failed to cast to topdown")))))

(fn `StartClock`
  (for _array_element (`self.Players`)
    (bind _asplayer_character (cast `/Game/Blueprints/Characters/PlayerCharacter` (`Controller.K2_GetPawn` _array_element))
      (:`then`
        (`AbilitySystemComponent.BP_ApplyGameplayEffectToTarget` :`self` (`self.AbilitySystem`) :`GameplayEffectClass` "/Game/GameplayAbilities/Effects/Times/GE_Day.GE_Day_C" :`Target` (`AbilitySystemBlueprintLibrary.GetAbilitySystemComponent` _asplayer_character) :`Level` 1.0))
      (:`CastFailed`
        (`KismetSystemLibrary.PrintString` "Failed to cast to topdown")))))

(fn `StopClock`
  (for _array_element (`self.Players`)
    (bind _asplayer_character (cast `/Game/Blueprints/Characters/PlayerCharacter` (`Controller.K2_GetPawn` _array_element))
      (:`then`
        (`AbilitySystemComponent.BP_ApplyGameplayEffectToTarget` :`self` (`self.AbilitySystem`) :`GameplayEffectClass` "/Game/GameplayAbilities/Effects/Times/GE_StopTime.GE_StopTime_C" :`Target` (`AbilitySystemBlueprintLibrary.GetAbilitySystemComponent` _asplayer_character) :`Level` 1.0))
      (:`CastFailed`
        (`KismetSystemLibrary.PrintString` "Failed to cast to topdown")))))

(fn `UserConstructionScript`)