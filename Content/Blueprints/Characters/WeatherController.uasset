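; Prototype weather controller that picks and times rain, thunderstorm, cloud or no-weather events, currently represented only by debug prints.
; ChoseNextWeather derives a randomized delay from ChaosLevel, then repeatedly filters a Probability map with weighted coin flips until fewer than two entries remain.
; WeatherCycle schedules StartWeatherEvent by timer, which in turn schedules a placeholder EndWeatherEvent.
; BeginPlay never starts the cycle, and Tick prints the current event.
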(event `self.ReceiveBeginPlay`
  (`KismetSystemLibrary.PrintString` "I was created" true true (struct :`R` 0.163957 :`G` 1.0 :`A` 1.0) 10.0))

(event `test`)

(event `self.ReceiveTick`
  (params (DeltaSeconds :type "Float (single-precision)"))
  (`KismetSystemLibrary.PrintString` (`self.weatherEvent`) true true (struct :`R` 1.0 :`G` 0.078564 :`B` 0.018841 :`A` 1.0) 0.0))

(fn `ChoseNextWeather`
  (locals (WeatherEventFound :type Boolean) (NumWeatherEvent :type Integer) (tmpList :type "Map of String to Float (double-precision)") (ProbabilityValue :type "Array of Float (double-precision)") (ProbabilityName :type "Array of String"))
  (bind _tmplist (`local.tmpList`))
  (bind _tmplist_2 (`local.tmpList`))
  (bind _probabilityname (`local.ProbabilityName`))
  (bind _returnvalue (`KismetArrayLibrary.Array_Length` _probabilityname))
  (bind _output (`|GetArrayItem` _probabilityname))
  (`KismetSystemLibrary.PrintString` "start to chose weather and time" true true (struct :`G` 1.0 :`B` 0.017494 :`A` 1.0) 10.0)
  ;[1 1 1] Choose when the next weather event will happen
  (switch `int` (`self.ChaosLevel`)
    (:`1`
      (set `self.InitialTime` 30))
    (:`2`
      (set `self.InitialTime` 20))
    (:`3`
      (set `self.InitialTime` 10)))
  (bind _output_get (set `self.TimeBeforeNextEvent` (+ (`KismetMathLibrary.FFloor` (* 10.0 (`KismetMathLibrary.RandomFloat`))) (`self.InitialTime`))))
  (`KismetSystemLibrary.PrintString` (`KismetStringLibrary.Conv_IntToString` _output_get) true true (struct :`R` 0.121427 :`G` 1.0 :`A` 1.0) 10.0)
  (set `local.tmpList` (`self.Probability`))
  (`KismetSystemLibrary.PrintString` "Starting the selection of the weather" true true (struct :`G` 1.0 :`B` 0.081037 :`A` 1.0) 10.0)
  (while (not (`local.WeatherEventFound`))
    (`KismetSystemLibrary.PrintString` (`KismetStringLibrary.Conv_IntToString` (`BlueprintMapLibrary.Map_Length` _tmplist)) true true (struct :`R` 0.226097 :`G` 1.0 :`A` 1.0) 10.0)
    (bind _values (`BlueprintMapLibrary.Map_Values` _tmplist))
    (set `local.ProbabilityValue` _values)
    (bind _keys (`BlueprintMapLibrary.Map_Keys` _tmplist_2))
    (set `local.ProbabilityName` _keys)
    (for _index (range (`BlueprintMapLibrary.Map_Length` _tmplist_2))
      (if (`KismetMathLibrary.RandomBoolWithWeight` (`|GetArrayItem` (`local.ProbabilityValue`) _index))
        (`KismetSystemLibrary.PrintString` "Event passed" true true (struct :`G` 1.0 :`B` 0.040609 :`A` 1.0) 10.0)
        (else
          (`BlueprintMapLibrary.Map_Remove` (`local.tmpList`) (`|GetArrayItem` (`local.ProbabilityName`) _index))
          (`KismetSystemLibrary.PrintString` "Event failed" true true (struct :`G` 1.0 :`B` 0.071678 :`A` 1.0) 10.0))))
    (if (< (`BlueprintMapLibrary.Map_Length` (`local.tmpList`)) 2)
      (set `local.WeatherEventFound` true)))
  (`KismetSystemLibrary.PrintString` "Event found" true true (struct :`R` 0.021898 :`G` 1.0 :`A` 1.0) 10.0)
  (`KismetSystemLibrary.PrintString` (`KismetStringLibrary.Conv_IntToString` _returnvalue) true true (struct :`G` 1.0 :`B` 0.026792 :`A` 1.0) 10.0)
  (if (== _returnvalue 0)
    (`KismetSystemLibrary.PrintString` "Nothing will happen" true true (struct :`G` 1.0 :`B` 0.026792 :`A` 1.0) 10.0)
    (set `self.WeatherEventChosen` "Nothing")
    (else
      (`KismetSystemLibrary.PrintString` "Theres a weather event" true true (struct :`G` 1.0 :`B` 0.026792 :`A` 1.0) 10.0)
      (`KismetSystemLibrary.PrintString` _output true true (struct :`G` 1.0 :`B` 0.026792 :`A` 1.0) 10.0)
      (set `self.WeatherEventChosen` _output))))

(fn `EndWeatherEvent`
  (params (WeatherEvent :type Boolean))
  ;[1 1 1] make event to destroy weather event
  (`KismetSystemLibrary.PrintString` "Destroy the weather event" true true (struct :`G` 1.0 :`B` 0.094754 :`A` 1.0) 10.0))

(fn `StartWeatherEvent`
  (bind _weathereventchosen (`self.WeatherEventChosen`))
  (switch `string` _weathereventchosen
    (:`Rain`
      (`KismetSystemLibrary.PrintString` "Its raining" true true (struct :`R` 0.057249 :`G` 1.0 :`A` 1.0) 10.0))
    (:`ThunderStorm`
      (`KismetSystemLibrary.PrintString` "ThunderStorm" true true (struct :`R` 0.136643 :`G` 1.0 :`A` 1.0) 10.0))
    (:`Clouds`
      (`KismetSystemLibrary.PrintString` "Clouds" true true (struct :`G` 1.0 :`B` 0.054792 :`A` 1.0) 10.0))
    (:`Nothing`
      (`KismetSystemLibrary.PrintString` "Nothing" true true (struct :`G` 1.0 :`B` 0.094417 :`A` 1.0) 10.0)))
  (set `self.weatherEvent` _weathereventchosen)
  (`KismetSystemLibrary.K2_SetTimer` null "EndWeatherEvent" 10.0))

(fn `UserConstructionScript`)

(fn `WeatherCycle`
  (`self.ChoseNextWeather`)
  (`KismetSystemLibrary.K2_SetTimer` null "StartWeatherEvent" (`KismetMathLibrary.Conv_IntToDouble` (`self.TimeBeforeNextEvent`))))